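; GM_LineDefence is the game mode for a wave-based line defence game, tracking state, score, wave number and kills.
; Bound events from the Player, DefenceLine and EnemyPoolManager trigger level-up, game over, and shop or game clear on wave clear.
; SetGameState broadcasts each change, starts waves, opens shop or results, and pauses through global time dilation.
; A zero-second delay before game over lets same-frame kill scores register before results display.
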(event `self.ReceiveBeginPlay`
  (set `PlayerController.bShowMouseCursor` true (`GameplayStatics.GetPlayerController` 0))
  (set `self.CurrentGameState` "NewEnumerator0"))

(event `self.ReceiveTick`
  (params (DeltaSeconds :type "Float (single-precision)")))

(event `BineEventLevelUp`
  ; Player 레벨업
  (add `/Game/Blueprints/Actors/Character/Player/BP_PlayerCharacter.OnChangedLevel` (`self.Player`) (`|CreateDelegate` :!event `LevelUp`)))

(event `LevelUp`
  ; Player 레벨업
  (`self.SetGameState` "NewEnumerator3"))

(event `/Game/Blueprints/BPI_ScoreInterface.AddGameScore`
  (params (InValue :type Integer))
  ; 게임 점수 갱신
  (bind _output_get (set `self.GameScore` (+ InValue (`self.GameScore`))))
  (`self.OnChangedGameScore` _output_get))

(event `BindEventGameOver`
  ; GameOver
  (add `/Game/Blueprints/Actors/Wall/BP_DefenceLine.OnGameOver` (`self.DefenceLine`) (`|CreateDelegate` :!event `GameOver`)))

(event `GameOver`
  ; GameOver
  ;; RaceCondition 해결용(디펜스바 hp가 0이 되서 Result  UI가 Score를 출력한 이후에 동일 프레임에 적 Death 처리가 되어 스코어가 갱신되면 MainHUD_Top의 스코어가 늦게 반영됨)
  (`KismetSystemLibrary.Delay` 0.0)
  (`self.SetGameState` "NewEnumerator4"))

(event `BIndEventWaveClear`
  ; 웨이브 클리어
  (add `/Game/Blueprints/Actors/BP_EnemyPoolManager.OnWaveClear` (`self.EnemyPoolManager`) (`|CreateDelegate` :!event `WaveClear`)))

(event `WaveClear`
  ; 웨이브 클리어
  (if (== (`self.TotalEnemyCount`) (`self.KillCount`))
    (`self.SetGameState` "NewEnumerator5")
    (else
      (`self.SetGameState` "NewEnumerator2"))))

(fn `IncreaseKillCount`
  (`/Engine/EditorBlueprintResources/StandardMacros.IncrementInt` (`self.KillCount`)))

(fn `SetGameState`
  (params (InNewState :type "/Game/Blueprints/Data/E_GameState Enum" :default "NewEnumerator0"))
  (bind _output_get (set `self.CurrentGameState` InNewState))
  (`self.OnChangedGameState` _output_get)
  (switch `/Game/Blueprints/Data/E_GameState` _output_get
    (:`NewEnumerator1`
      (`self.ToNextWave`)
      (`GameplayStatics.SetGlobalTimeDilation` 1.0))
    (:`NewEnumerator2`
      (`self.OpenShop`)
      (`GameplayStatics.SetGlobalTimeDilation` 0.0))
    (:`NewEnumerator3`
      (`KismetSystemLibrary.PrintString` "레벨업" true true (struct :`G` 0.04806 :`B` 1.0 :`A` 1.0))
      (`GameplayStatics.SetGlobalTimeDilation` 0.0))
    (:`NewEnumerator4`
      (`self.OpenResult` (`self.CurrentWaveNumber`) (`self.KillCount`) (`self.GameScore`) :!label _label)
      (`GameplayStatics.SetGlobalTimeDilation` 0.0))
    (:`NewEnumerator5`
      (goto _label))))

(fn `SetTotalEnemyCount`
  (params (InTotalCount :type Integer))
  (set `self.TotalEnemyCount` InTotalCount))

(fn `ToNextWave`
  (bind _result (`/Engine/EditorBlueprintResources/StandardMacros.IncrementInt` (`self.CurrentWaveNumber`))
    (:`  `
      (`/Game/Blueprints/Actors/BP_EnemyPoolManager.StartWave` (`self.EnemyPoolManager`) _result)
      (`self.OnWaveChanged`))))

(fn `UserConstructionScript`)
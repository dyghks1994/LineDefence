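; Object pool manager for the line-defence game that pre-spawns Normal and Fast enemies and releases them in waves.
; BeginPlay registers it with GM_LineDefence, fills both pools and starts the current wave.
; Each wave loads its spawn list from DT_WaveStage, and a looping timer activates pooled enemies at random Y positions between two side markers.
; ReturnEnemyToPool refills pools by type; temporary code chains waves after a delay.
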(event `self.ReceiveBeginPlay`
  ; 게임모드에 EnemyPoolManager 저장
  (bind _asgm_line_defence (cast `/Game/Blueprints/Framework/GameMode/GM_LineDefence` (`GameplayStatics.GetGameMode`))
    (:`then`
      (set `/Game/Blueprints/Framework/GameMode/GM_LineDefence.EnemyPoolManager` self _asgm_line_defence)
      ; 오프젝트 풀 초기화
      (for _ (range 1 (+ (`self.MaxPoolSize`) 1))
        (bind _returnvalue (`|SpawnActorFromClass` "/Game/Blueprints/Character/Enemy/BP_EnemyNormal.BP_EnemyNormal_C" (`KismetMathLibrary.MakeTransform` (`self.K2_GetActorLocation`)) "AlwaysSpawn" "MultiplyWithRoot" null null))
        (`KismetArrayLibrary.Array_Add` (`self.NormalEnemyPool`) _returnvalue)
        (bind _returnvalue_2 (`|SpawnActorFromClass` "/Game/Blueprints/Character/Enemy/BP_EnemyFast.BP_EnemyFast_C" (`KismetMathLibrary.MakeTransform` (`self.K2_GetActorLocation`)) "AlwaysSpawn" "MultiplyWithRoot" null null))
        (`KismetArrayLibrary.Array_Add` (`self.FastEnemyPool`) _returnvalue_2))
      (`self.StartWave` (`self.CurrentWaveNum`)))
    (:`CastFailed`
      (`KismetSystemLibrary.PrintString` "EnemyPoolManager 게임모드 세팅 실패" true true (struct :`R` 1.0 :`A` 1.0)))))

(event `StartWave`
  (params (InWaveNum :type Integer))
  (bind _returnvalue (`|GetDataTableRow` "/Game/Blueprints/Data/DT_WaveStage.DT_WaveStage" (`KismetStringLibrary.Conv_StringToName` (`KismetStringLibrary.BuildString_Int` "" "Wave" InWaveNum)))
    (:`then`
      (set `self.SpawnQueue` (break `/Game/Blueprints/Data/ST_WaveData` _returnvalue))
      (set `self.ElapsedTime` 0.0)
      (bind _returnvalue_2 (`KismetSystemLibrary.K2_SetTimerDelegate` (`|CreateDelegate` :!event `CheckSpawnQueue`) (`self.SpawnQueueCheckTime`) true))
      (set `self.WaveTimerHandle` _returnvalue_2))))

(event `CheckSpawnQueue`
  (bind _currentwavenum (`self.CurrentWaveNum`))
  (bind _spawnqueue (`self.SpawnQueue`))
  (bind (_output_spawntime _output_enemytype) (break `/Game/Blueprints/Data/ST_SpawnData` (`|GetArrayItem` _spawnqueue)))
  (set `self.ElapsedTime` (+ (`self.ElapsedTime`) (`self.SpawnQueueCheckTime`)))
  (if (> (`KismetArrayLibrary.Array_Length` _spawnqueue) 0)
    (if (>= (`self.ElapsedTime`) _output_spawntime)
      (`self.SpawnEnemyFromPool` _output_enemytype)
      (`KismetArrayLibrary.Array_Remove` _spawnqueue))
    (else
      (`KismetSystemLibrary.PrintString` (`KismetStringLibrary.BuildString_Int` "" "Wave" (`self.CurrentWaveNum`) "스폰 끝"))
      (`KismetSystemLibrary.K2_ClearAndInvalidateTimerHandle` (`self.WaveTimerHandle`))
      ; 임시 넥스트 웨이브 실행 코드
      (`KismetSystemLibrary.Delay` 5.0)
      (`/Engine/EditorBlueprintResources/StandardMacros.IncrementInt` _currentwavenum
        (:`  `
          (`self.StartWave` _currentwavenum))))))

(fn `AddEnemyToPool`
  (params (TargetPool :type "Array of /Game/Blueprints/BPI_Poolable Interface") (InEnemy :type "/Game/Blueprints/Character/Enemy/BP_EnemyBase Object Reference"))
  (`KismetArrayLibrary.Array_Add` TargetPool InEnemy))

(fn `ReturnEnemyToPool`
  (params (InEnemy :type "/Game/Blueprints/Character/Enemy/BP_EnemyBase Object Reference") (InType :type "/Game/Blueprints/Data/E_EnemyType Enum" :default "NewEnumerator0"))
  ; 활성 풀에서 제거
  (`KismetArrayLibrary.Array_Add` (`self.ActiveEnemies`) InEnemy)
  (if true
    ; EnemyType별 Pool로 회수
    (switch `/Game/Blueprints/Data/E_EnemyType` InType
      (:`NewEnumerator0`
        (`self.AddEnemyToPool` (`self.NormalEnemyPool`) InEnemy))
      (:`NewEnumerator1`
        (`self.AddEnemyToPool` (`self.FastEnemyPool`) InEnemy)))
    (else
      (`KismetSystemLibrary.PrintString` "Fail_EnemyPoolManager_ActivateEnemies Remove" true true (struct :`R` 1.0 :`A` 1.0)))))

(fn `SpawnEnemy_Fast`
  (bind (_returnvalue_x _returnvalue_y _returnvalue_z) (`KismetMathLibrary.BreakVector` (`self.K2_GetActorLocation`)))
  (bind _fastenemypool (`self.FastEnemyPool`))
  (bind _returnvalue (`KismetArrayLibrary.Array_LastIndex` _fastenemypool))
  (bind (_returnvalue_x_2 _returnvalue_y_2) (`KismetMathLibrary.BreakVector` (`self.K2_GetActorLocation` (`self.RightSide`))))
  (bind (_returnvalue_x_3 _returnvalue_y_3) (`KismetMathLibrary.BreakVector` (`self.K2_GetActorLocation` (`self.LeftSide`))))
  (bind _output (`|GetArrayItem` _fastenemypool _returnvalue))
  (if (> (`KismetArrayLibrary.Array_Length` (`self.FastEnemyPool`)) 0)
    ; 스폰 후 활성화 Enemy 배열에 add해서 관리
    (`/Game/Blueprints/BPI_Poolable.OnActivate` :`self` _output :`InLocation` (`KismetMathLibrary.MakeVector` _returnvalue_x (`KismetMathLibrary.RandomFloatInRange` _returnvalue_y_3 _returnvalue_y_2) _returnvalue_z))
    (`KismetArrayLibrary.Array_Add` (`self.ActiveEnemies`) _output)
    ; SpawnPool에서 제거
    (`KismetArrayLibrary.Array_Remove` _fastenemypool _returnvalue)
    (else
      ; PoolSize 체크
      (`KismetSystemLibrary.PrintString` "EnemyPool 부족" true true (struct :`R` 1.0 :`A` 1.0)))))

(fn `SpawnEnemy_Normal`
  (bind (_returnvalue_x _returnvalue_y _returnvalue_z) (`KismetMathLibrary.BreakVector` (`self.K2_GetActorLocation`)))
  (bind _normalenemypool (`self.NormalEnemyPool`))
  (bind _returnvalue (`KismetArrayLibrary.Array_LastIndex` _normalenemypool))
  (bind (_returnvalue_x_2 _returnvalue_y_2) (`KismetMathLibrary.BreakVector` (`self.K2_GetActorLocation` (`self.RightSide`))))
  (bind (_returnvalue_x_3 _returnvalue_y_3) (`KismetMathLibrary.BreakVector` (`self.K2_GetActorLocation` (`self.LeftSide`))))
  (bind _output (`|GetArrayItem` _normalenemypool _returnvalue))
  (if (> (`KismetArrayLibrary.Array_Length` (`self.NormalEnemyPool`)) 0)
    ; 스폰 후 활성화 Enemy 배열에 add해서 관리
    (`/Game/Blueprints/BPI_Poolable.OnActivate` :`self` _output :`InLocation` (`KismetMathLibrary.MakeVector` _returnvalue_x (`KismetMathLibrary.RandomFloatInRange` _returnvalue_y_3 _returnvalue_y_2) _returnvalue_z))
    (`KismetArrayLibrary.Array_Add` (`self.ActiveEnemies`) _output)
    ; SpawnPool에서 제거
    (`KismetArrayLibrary.Array_Remove` _normalenemypool _returnvalue)
    (else
      ; PoolSize 체크
      (`KismetSystemLibrary.PrintString` "EnemyPool 부족" true true (struct :`R` 1.0 :`A` 1.0)))))

(fn `SpawnEnemyFromPool`
  (params (InType :type "/Game/Blueprints/Data/E_EnemyType Enum" :default "NewEnumerator0"))
  (switch `/Game/Blueprints/Data/E_EnemyType` InType
    (:`NewEnumerator0`
      (`self.SpawnEnemy_Normal`))
    (:`NewEnumerator1`
      (`self.SpawnEnemy_Fast`))))

(fn `UserConstructionScript`)
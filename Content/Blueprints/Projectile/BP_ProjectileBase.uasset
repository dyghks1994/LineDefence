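; Base pooled projectile that starts dormant on BeginPlay and is reused through activate and deactivate events rather than spawned and destroyed.
; OnActivate restores visibility, tick and collision, places the actor, launches it along local X via ProjectileMovement at MoveSpeed, and starts a LifeTime timer.
; OnDeactivate hides it and disables tick and collision, without stopping movement.
; Sphere overlaps send a deactivate message to BP_EnemyBase actors, leaving the projectile active.
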(event `self.ReceiveBeginPlay`
  (`/Game/Blueprints/BPI_Poolable.OnDeactivate`))

(event `/Game/Blueprints/BPI_Poolable.OnActivate`
  (params (InLocation :type "Vector Structure") (InRotation :type "Rotator Structure"))
  ; ObjectPool에서 스폰할 때 활성화
  ;; 렌더, 틱, 충돌 설정
  (`self.SetActorHiddenInGame` false)
  (`self.SetActorTickEnabled` true)
  (`self.SetActorEnableCollision` true)
  ;; 스폰위치, 방향 설정
  (`MovementComponent.StopMovementImmediately` (`self.ProjectileMovement`))
  (`self.K2_SetActorLocationAndRotation` InLocation (`KismetMathLibrary.MakeRotator` 0.0 0.0 (.yaw InRotation)))
  (`ProjectileMovementComponent.SetVelocityInLocalSpace` (`self.ProjectileMovement`) (`KismetMathLibrary.MakeVector` (`self.MoveSpeed`)))
  ;; 발사체 유지시간 설정
  (bind _returnvalue (`KismetSystemLibrary.K2_SetTimerDelegate` (`|CreateDelegate` :!event `ReturnToPool`) (`self.LifeTIme`)))
  (set `self.LifeTImerHandle` _returnvalue))

(event `/Game/Blueprints/BPI_Poolable.OnDeactivate`
  ; 비활성화(렌더, 충돌, 이동 멈춤)
  (`self.SetActorHiddenInGame` true)
  (`self.SetActorTickEnabled` false)
  (`self.SetActorEnableCollision` false))

(event `self.SphereCollision.OnComponentBeginOverlap`
  (params (OverlappedComponent :type "PrimitiveComponent Object Reference") (OtherActor :type "Actor Object Reference") (OtherComp :type "PrimitiveComponent Object Reference") (OtherBodyIndex :type Integer) (bFromSweep :type Boolean) (SweepResult :type "HitResult Structure (by ref)"))
  (if (`KismetMathLibrary.ClassIsChildOf` (`GameplayStatics.GetObjectClass` OtherActor) "/Game/Blueprints/Character/BP_EnemyBase.BP_EnemyBase_C")
    (message `/Game/Blueprints/BPI_Poolable.OnDeactivate` OtherActor)))

(fn `GetAsActor`
  (returns (OutActor :type "Actor Object Reference"))
  (return self))

(fn `GetPoolableLocation`
  (returns (OutLocation :type "Vector Structure"))
  (return (0.0 0.0 0.0)))

(fn `UserConstructionScript`)
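; Enemy pool manager that pre-spawns Normal and Fast enemies on BeginPlay and runs timed waves from DT_WaveStage.
; A looping timer checks the wave's spawn queue and releases at most one due entry per tick.
; Each spawn pops the last pooled enemy of that type and activates it at a random Y between the side markers.
; An empty queue starts the next numbered wave after a delay.
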(event `self.ReceiveBeginPlay`
  (for _ (range 1 (+ (`self.MaxPoolSize`) 1))
    ; 오프젝트 풀 초기화
    (bind _returnvalue (`|SpawnActorFromClass` "/Game/Blueprints/Character/BP_EnemyNormal.BP_EnemyNormal_C" (`KismetMathLibrary.MakeTransform` (`self.K2_GetActorLocation`)) "Undefined" "MultiplyWithRoot" null null))
    (`KismetArrayLibrary.Array_Add` (`self.NormalEnemyPool`) _returnvalue)
    (bind _returnvalue_2 (`|SpawnActorFromClass` "/Game/Blueprints/Character/BP_EnemyFast.BP_EnemyFast_C" (`KismetMathLibrary.MakeTransform` (`self.K2_GetActorLocation`)) "Undefined" "MultiplyWithRoot" null null))
    (`KismetArrayLibrary.Array_Add` (`self.FastEnemyPool`) _returnvalue_2))
  (`self.StartWave` (`self.CurrentWaveNum`)))

(event `StartWave`
  (params (InWaveNum :type Integer))
  (bind _returnvalue (`|GetDataTableRow` "/Game/Blueprints/Data/DT_WaveStage.DT_WaveStage" (`KismetStringLibrary.Conv_StringToName` (`KismetStringLibrary.BuildString_Int` "" "Wave" InWaveNum)))
    (:`then`
      (set `self.SpawnQueue` (break `/Game/Blueprints/Data/ST_WaveData` _returnvalue))
      (set `self.ElapsedTime` 0.0)
      (bind _returnvalue_2 (`KismetSystemLibrary.K2_SetTimerDelegate` (`|CreateDelegate` :!event `CheckSpawnQueue`) (`self.SpawnQueueCheckTime`) true))
      (set `self.WaveTimerHandle` _returnvalue_2))))

(event `CheckSpawnQueue`
  (bind _currentwavenum (`self.CurrentWaveNum`))
  (bind _spawnqueue (`self.SpawnQueue`))
  (bind (_output_spawntime _output_enemytype) (break `/Game/Blueprints/Data/ST_SpawnData` (`|GetArrayItem` _spawnqueue)))
  (set `self.ElapsedTime` (+ (`self.ElapsedTime`) (`self.SpawnQueueCheckTime`)))
  (if (> (`KismetArrayLibrary.Array_Length` _spawnqueue) 0)
    (if (>= (`self.ElapsedTime`) _output_spawntime)
      (`self.SpawnEnemyFromPool` _output_enemytype)
      (`KismetArrayLibrary.Array_Remove` _spawnqueue))
    (else
      (`KismetSystemLibrary.PrintString` (`KismetStringLibrary.BuildString_Int` "" "Wave" (`self.CurrentWaveNum`) "스폰 끝"))
      (`KismetSystemLibrary.K2_ClearAndInvalidateTimerHandle` (`self.WaveTimerHandle`))
      (`KismetSystemLibrary.Delay` 5.0)
      (`/Engine/EditorBlueprintResources/StandardMacros.IncrementInt` _currentwavenum
        (:`  `
          (`self.StartWave` _currentwavenum))))))

(fn `ExecuteSpawnFromPool`
  (params (TargetPool :type "Array of /Game/Blueprints/BPI_Poolable Interface"))
  (bind _returnvalue (`KismetArrayLibrary.Array_LastIndex` TargetPool))
  (bind (_returnvalue_x _returnvalue_y _returnvalue_z) (`KismetMathLibrary.BreakVector` (`self.K2_GetActorLocation`)))
  (bind (_returnvalue_x_2 _returnvalue_y_2) (`KismetMathLibrary.BreakVector` (`self.K2_GetActorLocation` (`self.RightSide`))))
  (bind (_returnvalue_x_3 _returnvalue_y_3) (`KismetMathLibrary.BreakVector` (`self.K2_GetActorLocation` (`self.LeftSide`))))
  (`/Game/Blueprints/BPI_Poolable.OnActivate` (`|GetArrayItem` TargetPool _returnvalue) (`KismetMathLibrary.MakeVector` _returnvalue_x (`KismetMathLibrary.RandomFloatInRange` _returnvalue_y_3 _returnvalue_y_2) _returnvalue_z))
  (`KismetArrayLibrary.Array_Remove` TargetPool _returnvalue))

(fn `SpawnEnemyFromPool`
  (params (InType :type "/Game/Blueprints/Data/E_EnemyType Enum" :default "NewEnumerator0"))
  (switch `/Game/Blueprints/Data/E_EnemyType` InType
    (:`NewEnumerator0`
      (`self.ExecuteSpawnFromPool` (`self.NormalEnemyPool`)))
    (:`NewEnumerator1`
      (`self.ExecuteSpawnFromPool` (`self.FastEnemyPool`)))))

(fn `UserConstructionScript`)
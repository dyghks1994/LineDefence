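; BP_EnemyBase is a pooled enemy character that advances toward the player's defence line.
; Activation places it, enables tick and collision, starts an attack-cooldown timer, sets walk speed and issues AI MoveTo along X.
; Attack halts movement for the cooldown, re-arms its timer and resumes the advance; it applies no damage here.
; Deactivate, also run on BeginPlay, disables tick and collision and stops movement, but leaves the actor visible.
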(event `self.ReceiveBeginPlay`
  (`self.Deactivate`))

(event `Activate`
  (params (InLocation :type "Vector Structure"))
  ; ObjectPool에서 스폰할 때 활성화
  ;; 렌더, 틱, 충돌 설정
  (`self.SetActorHiddenInGame` false)
  (`self.SetActorTickEnabled` true)
  (`self.SetActorEnableCollision` true)
  (`self.K2_SetActorLocation` InLocation)
  ;; 공격 주기 설정
  (bind _returnvalue (`KismetSystemLibrary.K2_SetTimerDelegate` (`|CreateDelegate` :!event `Attack`) (`self.AttackCoolDown`)))
  (set `self.AttackTimerHandle` _returnvalue)
  ;; 이동속도 설정
  (set `CharacterMovementComponent.MaxWalkSpeed` (`self.MoveSpeed`) (`self.CharacterMovement`))
  (`self.MoveToDefenceLine`))

(event `Attack`
  (if (not (`self.bIsAttacking`))
    (set `self.bIsAttacking` true)
    (`KismetSystemLibrary.K2_ClearAndInvalidateTimerHandle` (`self.AttackTimerHandle`))
    (`MovementComponent.StopMovementImmediately` (`self.CharacterMovement`))
    (`KismetSystemLibrary.Delay` (`self.AttackCoolDown`))
    (set `self.bIsAttacking` false)
    (`KismetSystemLibrary.K2_SetTimerDelegate` (delegate `Attack`) (`self.AttackCoolDown`))
    (`self.MoveToDefenceLine`)))

(event `MoveToDefenceLine`
  (bind (_returnvalue_x _returnvalue_y _returnvalue_z) (`KismetMathLibrary.BreakVector` (`self.K2_GetActorLocation`)))
  ; 플레이어 방어라인으로 이동 설정
  (`|AIMoveTo` self (`KismetMathLibrary.MakeVector` (`self.TargetPosX`) _returnvalue_y _returnvalue_z) null))

(event `self.ReceiveTick`
  (params (DeltaSeconds :type "Float (single-precision)")))

(event `/Game/Blueprints/BPI_Poolable.OnActivate`
  (params (InLocation :type "Vector Structure"))
  (`self.Activate` InLocation))

(event `/Game/Blueprints/BPI_Poolable.OnDeactivate`
  (`self.Deactivate`))

(fn `Deactivate`
  ; 비활성화(렌더, 충돌, 이동 멈춤)
  (`self.SetActorHiddenInGame` false)
  (`self.SetActorTickEnabled` false)
  (`self.SetActorEnableCollision` false)
  (`Controller.StopMovement` (`AIBlueprintHelperLibrary.GetAIController` null)))

(fn `UserConstructionScript`)
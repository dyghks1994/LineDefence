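; Normal enemy variant for the line-defence mode that sets its enemy type on BeginPlay and fires pooled projectiles.
; Its OnFire override calls the parent, then spawns one projectile from EnemyProjectilePoolManager at MuzzleAnchor along the actor's forward vector.
; An invalid pool reference is refetched from GM_LineDefence, printing an error if that cast fails.
; The burst loop runs once, and the burst-delay timer and older fire-request nodes are unwired.
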(event `self.ReceiveBeginPlay`
  (`parent.ReceiveBeginPlay`)
  (set `self.MyEnemyType` "NewEnumerator0"))

(event `TriggerSpawnProjectile`)

(fn `OnFire`
  (`parent.OnFire`)
  ; 연사를 해야 한다면
  (for _ (range 1)
    ; forward 방향으로 발사체 스폰요청
    (`/Engine/EditorBlueprintResources/StandardMacros.IsValid` (`self.EnemyProjectilePoolManager`)
      (:`Is Valid`
        (`/Game/Blueprints/BP_EnemyProjectilePoolManager.SpawnProjectileFromPool` (`self.EnemyProjectilePoolManager`) (`SceneComponent.K2_GetComponentLocation` (`self.MuzzleAnchor`)) (`KismetMathLibrary.MakeRotFromX` (`self.GetActorForwardVector`)) "NewEnumerator0" :!label _label))
      (:`Is Not Valid`
        (bind _asgm_line_defence (cast `/Game/Blueprints/Framework/GameMode/GM_LineDefence` (`GameplayStatics.GetGameMode`))
          (:`then`
            (set `self.EnemyProjectilePoolManager` (`/Game/Blueprints/Framework/GameMode/GM_LineDefence.EnemyProjectilePoolManager` _asgm_line_defence))
            (goto _label))
          (:`CastFailed`
            (`KismetSystemLibrary.PrintString` "EnemyProjectilePool 세팅 실패" true true (struct :`R` 1.0 :`A` 1.0) 5.0)))))))

(fn `UserConstructionScript`
  (`parent.UserConstructionScript`))
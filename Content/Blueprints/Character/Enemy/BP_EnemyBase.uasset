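; Base pooled enemy for a line-defence game that walks toward the player's defence line and periodically pauses to attack.
; BeginPlay caches the enemy and projectile pool managers from GM_LineDefence, then deactivates the enemy until it is activated from the pool.
; Activation restores visibility, tick and collision, then starts movement and a cooldown timer; attacks halt movement and call an empty OnFire hook.
; ReturntoPool deactivates it and hands it back by enemy type.
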(event `self.ReceiveBeginPlay`
  (bind _asgm_line_defence (cast `/Game/Blueprints/Framework/GameMode/GM_LineDefence` (`GameplayStatics.GetGameMode`))
    (:`then`
      (set `self.EnemyPoolManager` (`/Game/Blueprints/Framework/GameMode/GM_LineDefence.EnemyPoolManager` _asgm_line_defence))
      (set `self.EnemyProjectilePoolManager` (`/Game/Blueprints/Framework/GameMode/GM_LineDefence.EnemyProjectilePoolManager` _asgm_line_defence))
      (`self.Deactivate`))
    (:`CastFailed`
      (`KismetSystemLibrary.PrintString` "EnemyBase 매니저 세팅 실패" true true (struct :`R` 1.0 :`A` 1.0) 5.0))))

(event `Activate`
  (params (InLocation :type "Vector Structure"))
  ; ObjectPool에서 스폰할 때 활성화
  ;; 렌더, 틱, 충돌 설정
  (`self.SetActorHiddenInGame` false)
  (`self.SetActorTickEnabled` true)
  (`self.SetActorEnableCollision` true)
  (`self.K2_SetActorLocation` InLocation)
  ;; 공격 주기 설정
  (bind _returnvalue (`KismetSystemLibrary.K2_SetTimerDelegate` (`|CreateDelegate` :!event `Attack`) (`self.AttackCoolDown`)))
  (set `self.AttackTimerHandle` _returnvalue)
  ;; 이동속도 설정
  (set `CharacterMovementComponent.MaxWalkSpeed` (`self.MoveSpeed`) (`self.CharacterMovement`))
  (`self.MoveToDefenceLine`))

(event `Attack`
  (if (not (`self.bIsAttacking`))
    (set `self.bIsAttacking` true)
    (`KismetSystemLibrary.K2_ClearAndInvalidateTimerHandle` (`self.AttackTimerHandle`))
    (`MovementComponent.StopMovementImmediately` (`self.CharacterMovement`))
    (`self.OnFire`)
    (`KismetSystemLibrary.Delay` (`self.AttackCoolDown`))
    (set `self.bIsAttacking` false)
    (`KismetSystemLibrary.K2_SetTimerDelegate` (delegate `Attack`) (`self.AttackCoolDown`))
    (`self.MoveToDefenceLine`)))

(event `MoveToDefenceLine`
  (bind (_returnvalue_x _returnvalue_y _returnvalue_z) (`KismetMathLibrary.BreakVector` (`self.K2_GetActorLocation`)))
  ; 플레이어 방어라인으로 이동 설정
  (`|AIMoveTo` self (`KismetMathLibrary.MakeVector` (`self.TargetPosX`) _returnvalue_y _returnvalue_z) null))

(event `self.ReceiveTick`
  (params (DeltaSeconds :type "Float (single-precision)")))

(event `/Game/Blueprints/BPI_Poolable.OnActivate`
  (params (InLocation :type "Vector Structure") (InRotation :type "Rotator Structure"))
  (`self.Activate` InLocation))

(event `/Game/Blueprints/BPI_Poolable.OnDeactivate`
  (`self.Deactivate`))

(event `/Game/Blueprints/BPI_Poolable.ReturnToPool`
  (bind _enemypoolmanager (`self.EnemyPoolManager`))
  (`/Game/Blueprints/BPI_Poolable.OnDeactivate`)
  ; SpawnPoolManager에 다시 추가
  (`/Engine/EditorBlueprintResources/StandardMacros.IsValid` _enemypoolmanager
    (:`Is Valid`
      (`/Game/Blueprints/BP_EnemyPoolManager.ReturnEnemyToPool` _enemypoolmanager self (`self.MyEnemyType`)))))

(fn `Deactivate`
  (bind _returnvalue (`AIBlueprintHelperLibrary.GetAIController` null))
  ; 비활성화(렌더, 충돌, 이동 멈춤)
  (`/Engine/EditorBlueprintResources/StandardMacros.IsValid` _returnvalue
    (:`Is Valid`
      (`Controller.StopMovement` _returnvalue))
    (:`Is Not Valid`
      _))
  (`self.SetActorHiddenInGame` true)
  (`self.SetActorTickEnabled` false)
  (`self.SetActorEnableCollision` false))

(fn `GetAsActor`
  (returns (OutActor :type "Actor Object Reference"))
  (return null))

(fn `GetPoolableLocation`
  (returns (OutLocation :type "Vector Structure"))
  (return (`self.K2_GetActorLocation`)))

(fn `OnFire`)

(fn `UserConstructionScript`)
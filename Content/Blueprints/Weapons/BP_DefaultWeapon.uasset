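; BP_DefaultWeapon is the default weapon for the line-defence mode, currently aiming at enemies, with firing only stubbed as a debug print.
; BeginPlay caches the enemy and player-projectile pool managers from GM_LineDefence and starts a looping attack-cooldown timer.
; Tick scans the pool's active enemies by squared distance and turns WeaponMesh, yaw only, toward the nearest.
; The projectile pool is cached and validated but not yet used.
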(event `self.ReceiveBeginPlay`
  (bind _asgm_line_defence (cast `/Game/Blueprints/Framework/GameMode/GM_LineDefence` (`GameplayStatics.GetGameMode`)))
  (bind _output_get (set `self.EnemyPoolManager` (`/Game/Blueprints/Framework/GameMode/GM_LineDefence.EnemyPoolManager` _asgm_line_defence)))
  (`/Engine/EditorBlueprintResources/StandardMacros.IsValid` _output_get
    (:`Is Valid`
      (`KismetSystemLibrary.PrintString` "DefaultWeapon : EnemyPoolManager 세팅 O" true true (struct :`B` 1.0 :`A` 1.0) 5.0)
      (bind _output_get_2 (set `self.PlayerProjectilePoolManager` (`/Game/Blueprints/Framework/GameMode/GM_LineDefence.PlayerProjectilePoolManager` _asgm_line_defence)))
      (`/Engine/EditorBlueprintResources/StandardMacros.IsValid` _output_get_2
        (:`Is Valid`
          (`KismetSystemLibrary.PrintString` (`KismetStringLibrary.Concat_StrStr` (`KismetSystemLibrary.GetDisplayName` self) "PlayerProjectilePoolManager 세팅 O") true true (struct :`B` 1.0 :`A` 1.0) 5.0)
          (`KismetSystemLibrary.K2_SetTimerDelegate` (`|CreateDelegate` :!event `OnFire`) (`self.AttackCoolDown`) true))
        (:`Is Not Valid`
          (`KismetSystemLibrary.PrintString` (`KismetStringLibrary.Concat_StrStr` (`KismetSystemLibrary.GetDisplayName` self) "PlayerProjectilePoolManager 세팅 X") true true (struct :`R` 1.0 :`A` 1.0) 5.0))))
    (:`Is Not Valid`
      (`KismetSystemLibrary.PrintString` "DefaultWeapon : EnemyPoolManager 세팅 X" true true (struct :`R` 1.0 :`A` 1.0) 5.0))))

(event `self.ReceiveTick`
  (params (DeltaSeconds :type "Float (single-precision)"))
  (bind _enemypoolmanager (`self.EnemyPoolManager`))
  (bind _targetactor (`self.TargetActor`))
  ; 가장 가까운 Enemy 계산
  (set `self.CurrentTargetDistance` 9999999.0)
  (set `self.TargetActor` null)
  (`/Engine/EditorBlueprintResources/StandardMacros.IsValid` _enemypoolmanager
    (:`Is Valid`
      (for _array_element (`/Game/Blueprints/BP_EnemyPoolManager.ActiveEnemies` _enemypoolmanager)
        (bind _outlocation (`/Game/Blueprints/BPI_Poolable.GetPoolableLocation` _array_element))
        (bind _returnvalue (`KismetMathLibrary.Vector_DistanceSquared` _outlocation (`self.K2_GetActorLocation`)))
        (if (< _returnvalue (`self.CurrentTargetDistance`))
          (set `self.CurrentTargetDistance` _returnvalue)
          (set `self.TargetActor` _array_element)))
      ; 렌더용 디폴트 무기 회전
      (`/Engine/EditorBlueprintResources/StandardMacros.IsValid` (`KismetSystemLibrary.Conv_InterfaceToObject` _targetactor)
        (:`Is Valid`
          (bind _outlocation_2 (`/Game/Blueprints/BPI_Poolable.GetPoolableLocation` _targetactor))
          (`SceneComponent.K2_SetWorldRotation` (`self.WeaponMesh`) (`KismetMathLibrary.MakeRotator` 0.0 0.0 (.yaw (`KismetMathLibrary.FindLookAtRotation` (`self.K2_GetActorLocation`) _outlocation_2))) false false))))))

(event `OnFire`
  (`KismetSystemLibrary.PrintString` (`KismetStringLibrary.Concat_StrStr` (`KismetSystemLibrary.GetDisplayName` self) ": OnFire") true true (struct :`R` 0.006927 :`G` 1.0 :`B` 0.058445 :`A` 1.0)))

(fn `UserConstructionScript`)
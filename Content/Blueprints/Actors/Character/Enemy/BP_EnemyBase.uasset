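; Pooled base enemy for a line-defence game that walks to the defence line via AI Move To.
; Activation applies spawn stats and enables the actor; deactivation hides and stops it.
; Within X-axis range, Tick uses a cooldown to randomly attack or move, with delays around an empty OnFire hook.
; Hits roll criticals and spawn damage text; death grants EXP and score, then returns it to the pool, guarded against repeats.
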(event `self.ReceiveBeginPlay`
  (bind _asgm_line_defence (cast `/Game/Blueprints/Framework/GameMode/GM_LineDefence` (`GameplayStatics.GetGameMode`))
    (:`then`
      (set `self.GM_LineDefence` _asgm_line_defence)
      (set `self.EnemyPoolManager` (`/Game/Blueprints/Framework/GameMode/GM_LineDefence.EnemyPoolManager` _asgm_line_defence))
      (set `self.EnemyProjectilePoolManager` (`/Game/Blueprints/Framework/GameMode/GM_LineDefence.EnemyProjectilePoolManager` _asgm_line_defence))
      (`self.Deactivate`))
    (:`CastFailed`
      (`KismetSystemLibrary.PrintString` "EnemyBase 매니저 세팅 실패" true true (struct :`R` 1.0 :`A` 1.0) 5.0))))

(event `Activate`
  (params (InLocation :type "Vector Structure"))
  ; ObjectPool에서 스폰할 때 활성화
  ;; 렌더, 틱, 충돌 설정
  (`self.SetActorHiddenInGame` false)
  (`self.SetActorTickEnabled` true)
  (`self.SetActorEnableCollision` true)
  (`self.K2_SetActorLocation` InLocation)
  ;; 중복리턴 방지용 bool 변수
  (set `self.bIsReturningToPool` false)
  (`self.MoveToDefenceLine`))

(event `Attack`
  (if (not (`self.bIsAttacking`))
    (set `self.bIsAttacking` true)
    (`MovementComponent.StopMovementImmediately` (`self.CharacterMovement`))
    ; 선딜레이
    (`KismetSystemLibrary.Delay` (`KismetMathLibrary.RandomFloatInRange` 0.5 1.0))
    ; 사격
    (`self.OnFire`)
    ; 후딜레이
    (`KismetSystemLibrary.Delay` (`KismetMathLibrary.RandomFloatInRange` 1.0 1.5))
    (set `self.AttackCoolTImeTimer` (`self.AttackCoolTIme`))
    (set `self.bIsAttacking` false)))

(event `self.ReceiveTick`
  (params (DeltaSeconds :type "Float (single-precision)"))
  (bind _attackcooltimetimer (`self.AttackCoolTImeTimer`))
  (bind _y (.y (`self.K2_GetActorLocation`)))
  ; 공격 사거리 판정
  (if (< (`KismetMathLibrary.Distance2D` (`KismetMathLibrary.MakeVector2D` (.x (`self.K2_GetActorLocation`)) _y) (`KismetMathLibrary.MakeVector2D` (`self.TargetPosX`) _y)) (`self.AttackRange`))
    (if (> _attackcooltimetimer 0.0)
      (set `self.AttackCoolTImeTimer` (- _attackcooltimetimer (`GameplayStatics.GetWorldDeltaSeconds`)))
      (elif (not (`self.bIsAttacking`))
        ; 일정확률로 공격 or 이동
        (if (< (`KismetMathLibrary.RandomIntegerInRange` 1 10) 2)
          (`self.MoveToDefenceLine`)
          (set `self.AttackCoolTImeTimer` 2.0)
          (else
            (`self.Attack`)))))))

(event `MoveToDefenceLine`
  (bind (_returnvalue_x _returnvalue_y _returnvalue_z) (`KismetMathLibrary.BreakVector` (`self.K2_GetActorLocation`)))
  ; 플레이어 방어라인으로 이동 설정
  (`|AIMoveTo` self (`KismetMathLibrary.MakeVector` (`self.TargetPosX`) _returnvalue_y _returnvalue_z) null))

(event `/Game/Blueprints/BPI_Poolable.OnActivate`
  (params (InLocation :type "Vector Structure") (InRotation :type "Rotator Structure") (InStat :type "/Game/Blueprints/Data/SpawnData/ST_EnemyStat Structure"))
  (`self.SetSpawnStat` InStat)
  (`self.Activate` InLocation))

(event `/Game/Blueprints/BPI_Poolable.OnDeactivate`
  (`self.Deactivate`))

(event `/Game/Blueprints/BPI_Poolable.ReturnToPool`
  (bind _enemypoolmanager (`self.EnemyPoolManager`))
  (`/Game/Blueprints/BPI_Poolable.OnDeactivate`)
  (set `self.bIsReturningToPool` true)
  ; SpawnPoolManager에 다시 추가
  (`/Engine/EditorBlueprintResources/StandardMacros.IsValid` _enemypoolmanager
    (:`Is Valid`
      (`/Game/Blueprints/Actors/BP_EnemyPoolManager.ReturnEnemyToPool` _enemypoolmanager self (`self.MyEnemyType`)))))

(event `/Game/Blueprints/BPI_HasHp.OnHit`
  (params (InDamage :type Integer))
  (bind _returnvalue (`GameplayStatics.GetPlayerPawn` 0))
  (bind _applydamage (`self.ApplyDamage`))
  (bind _gm_linedefence (`self.GM_LineDefence`))
  (if (not (`self.bIsReturningToPool`))
    ; 랜덤 크리티컬 적용
    (if (<= (`KismetMathLibrary.RandomIntegerInRange` 1 10) 3)
      (set `self.ApplyDamage` (* InDamage 2))
      (`self.SpawnDamageTextActor` _applydamage true)
      (else
        (set `self.ApplyDamage` InDamage)
        (`self.SpawnDamageTextActor` _applydamage)))
    ; 대미지 적용
    (set `self.CurrentHp` (`KismetMathLibrary.Max` (- (`self.CurrentHp`) (`self.ApplyDamage`))))
    (if (== (`self.CurrentHp`) 0)
      (if (`KismetSystemLibrary.DoesImplementInterface` _returnvalue "/Game/Blueprints/BPI_HasLvAndExp.BPI_HasLvAndExp_C")
        (message `/Game/Blueprints/BPI_HasLvAndExp.IncreaseExp` _returnvalue (`self.ExpReward`))
        (if (`KismetSystemLibrary.DoesImplementInterface` _gm_linedefence "/Game/Blueprints/BPI_ScoreInterface.BPI_ScoreInterface_C")
          (`/Game/Blueprints/BPI_ScoreInterface.AddGameScore` _gm_linedefence (`self.ScoreReward`))
          (`self.ReturnToPool`))))))

(fn `Deactivate`
  (bind _returnvalue (`AIBlueprintHelperLibrary.GetAIController` null))
  ; 비활성화(렌더, 충돌, 이동 멈춤)
  (`/Engine/EditorBlueprintResources/StandardMacros.IsValid` _returnvalue
    (:`Is Valid`
      (`Controller.StopMovement` _returnvalue))
    (:`Is Not Valid`
      _))
  (`self.SetActorHiddenInGame` true)
  (`self.SetActorTickEnabled` false)
  (`self.SetActorEnableCollision` false)
  ;; 중복리턴 방지용 체크 세팅
  (set `self.bIsReturningToPool` true)
  ;; 공격 타이머 클리어
  (`KismetSystemLibrary.K2_ClearAndInvalidateTimerHandle` (`self.AttackTimerHandle`)))

(fn `GetAsActor`
  (returns (OutActor :type "Actor Object Reference"))
  (return null))

(fn `GetPoolableLocation`
  (returns (OutLocation :type "Vector Structure"))
  (return (`self.K2_GetActorLocation`)))

(fn `OnFire`)

(fn `SetSpawnStat`
  (params (InStat :type "/Game/Blueprints/Data/SpawnData/ST_EnemyStat Structure"))
  (bind (_basehp _basespeed _statmultiplier) (break `/Game/Blueprints/Data/SpawnData/ST_EnemyStat` InStat))
  ; HP 설정
  (bind _output_get (set `self.MaxHp` (* (`KismetMathLibrary.Conv_IntToDouble` _basehp) (+ 1.0 _statmultiplier))))
  (set `self.CurrentHp` _output_get)
  ; 이동속도 설정
  (set `CharacterMovementComponent.MaxWalkSpeed` (+ (`self.MoveSpeed`) (* 0.05 _basespeed)) (`self.CharacterMovement`))
  ; 처치 시 보상 점수 세팅
  (set `self.ScoreReward` (`self.MaxHp`)))

(fn `SpawnDamageTextActor`
  (params (InDamage :type Integer) (isCritial :type Boolean))
  ; 데미지 텍스트 UI 방법 (2) - 위젯 스폰용 액터 스폰
  (bind _returnvalue (`|SpawnActorFromClass` "/Game/Blueprints/Framework/UI/DamageText/BP_DamageTextActor.BP_DamageTextActor_C" (`KismetMathLibrary.MakeTransform` (+ (`self.K2_GetActorLocation`) (`KismetMathLibrary.MakeVector` 0.0 0.0 50.0)) (`self.K2_GetActorRotation`)) "Undefined" "MultiplyWithRoot" null null))
  (`/Game/Blueprints/Framework/UI/DamageText/BP_DamageTextActor.SetDamageText` _returnvalue InDamage isCritial))

(fn `UserConstructionScript`)
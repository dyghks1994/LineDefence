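; Player inventory component that keeps a list of weapons, with an unfinished grid-based placement system.
; AddWeapon appends entries with valid weapon data and broadcasts the updated list through OnInventoryUpdate, while ClearWeaponList empties it without broadcasting.
; The grid logic is stubbed: occupancy map setup on BeginPlay has empty loops, TryAddWeapon walks shape cells but always succeeds, and GetUniqueWeaponList is empty.
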(event `self.ReceiveBeginPlay`
  (for _index (range 0)
    (for _index_2 (range 0)
      _)))

(event `/Game/Blueprints/BPI_HasWeapon.AddWeapon`
  (params (InWeapon :type "/Game/Blueprints/Data/InventoryData/ST_WeaponInstance Structure"))
  (bind _weaponlist (`self.WeaponList`))
  (`/Engine/EditorBlueprintResources/StandardMacros.IsValid` (`.WeaponData_2_806B7AB84D1E9159DF97DF868F631B6D` (break `/Game/Blueprints/Data/InventoryData/ST_WeaponInstance` InWeapon))
    (:`Is Valid`
      (`KismetArrayLibrary.Array_Add` _weaponlist InWeapon)
      (`self.OnInventoryUpdate` _weaponlist))))

(event `/Game/Blueprints/BPI_HasWeapon.ClearWeaponList`
  (bind _weaponlist (`self.WeaponList`))
  (for _array_element _weaponlist
    (`KismetArrayLibrary.Array_RemoveItem` _weaponlist _array_element))
  (`KismetArrayLibrary.Array_Clear` _weaponlist))

(fn `GetUniqueWeaponList`)

(fn `TryAddWeapon`
  (params (InWeaponData :type "/Game/Blueprints/Data/InventoryData/OldVerBackup/ST_WeaponData_Old Structure") (OriginPosition :type "Vector2D Structure"))
  (returns (Success :type Boolean))
  (bind _cells (break `/Game/Blueprints/Data/InventoryData/OldVerBackup/ST_WeaponShape_Old` (`.WeaponShape_18_BE5C6A4D4A3EB9A4FE6C0BA38DA79F14` (break `/Game/Blueprints/Data/InventoryData/OldVerBackup/ST_WeaponData_Old` InWeaponData))))
  (for _array_element _cells
    _)
  (for _array_element_2 _cells
    _)
  (return true))
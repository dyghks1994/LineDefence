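; BP_PlayerCharacter is the player character Blueprint, handling experience, leveling and a debug weapon spawn.
; IncreaseExp adds experience, broadcasts percent and ratio through OnChangedExp, and calls LevelUp once MaxExp is reached.
; LevelUp raises Level, broadcasts the change and resets experience to zero, discarding overflow and leaving MaxExp unchanged.
; A debug key spawns a BP_WeaponPierce snapped to WeaponAnchor and prints a test message.
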(event EventBeginPlay)

(event Collision|EventActorBeginOverlap
  (params (OtherActor :type Actor%20Object%20Reference)))

(event EventTick
  (params (DeltaSeconds :type Float%20%28single-precision%29)))

(event EventIncreaseExp
  (params (InExp :type Integer))
  (bind _output_get (Variables|Default|SetCurrentExp (+ InExp (Variables|Default|GetCurrentExp))))
  (Default|CallOnChangedExp (* (/ (Math|Conversions|ToFloat(Integer) _output_get) (Math|Conversions|ToFloat(Integer) (Variables|Default|GetMaxExp))) 1e+02) (/ (Math|Conversions|ToFloat(Integer) _output_get) (Math|Conversions|ToFloat(Integer) (Variables|Default|GetMaxExp))))
  (if (>= (Variables|Default|GetCurrentExp) (Variables|Default|GetMaxExp))
    (CallFunction|LevelUp)))

(event Input|KeyboardEvents|DebugKey1
  (params (Key :type Key%20Structure :default "None") (ActionValue :type Input%20Action%20Value%20Structure))
  (:Pressed
    (bind _returnvalue (Game|SpawnActorfromClass "/Game/Blueprints/Actors/Weapons/BP_WeaponPierce.BP_WeaponPierce_C" (Transformation|GetWorldTransform (Variables|Default|GetWeaponAnchor)) "AlwaysSpawn" "MultiplyWithRoot" 0 0))
    (Transformation|AttachComponentToComponent _returnvalue (Variables|Default|GetWeaponAnchor) "None" "SnapToTarget" "SnapToTarget" "SnapToTarget" true)
    (Development|PrintString "테스트 무기 추가")))

(fn ConstructionScript)

(fn LevelUp
  (Math|Integer|IncrementInt (Variables|Default|GetLevel)
    (:%20%20
      (Default|CallOnChangedLevel)
      (bind _output_get (Variables|Default|SetCurrentExp 0))
      (Default|CallOnChangedExp (Math|Conversions|ToFloat(Integer) _output_get) (Math|Conversions|ToFloat(Integer) _output_get)))))
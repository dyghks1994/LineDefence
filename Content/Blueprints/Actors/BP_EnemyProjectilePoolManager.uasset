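; Object pool manager actor that supplies Normal and Fast enemy projectiles in the line defence game mode.
; On BeginPlay it registers itself with GM_LineDefence, then pre-spawns MaxPoolSize projectiles of each type at its own location.
; SpawnProjectileFromPool activates and removes the last projectile of the requested type at the muzzle transform, doing nothing when that pool is empty.
; ReturnProjectileToPool adds a projectile back to the array matching its type.
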(event `self.ReceiveBeginPlay`
  ; 게임모드에 EnemyProjectileManager 저장
  (bind _asgm_line_defence (cast `/Game/Blueprints/Framework/GameMode/GM_LineDefence` (`GameplayStatics.GetGameMode`))
    (:`then`
      (set `/Game/Blueprints/Framework/GameMode/GM_LineDefence.EnemyProjectilePoolManager` self _asgm_line_defence)
      ; Pool 초기화
      (for _ (range 1 (+ (`self.MaxPoolSize`) 1))
        (bind _returnvalue (`|SpawnActorFromClass` "/Game/Blueprints/Actors/Projectile/EnemyProjectile/BP_EnemyProjectile_Normal.BP_EnemyProjectile_Normal_C" (`KismetMathLibrary.MakeTransform` (`self.K2_GetActorLocation`)) "AlwaysSpawn" "MultiplyWithRoot" null null))
        (`KismetArrayLibrary.Array_Add` (`self.EnemyProjectilePool_Normal`) _returnvalue)
        (bind _returnvalue_2 (`|SpawnActorFromClass` "/Game/Blueprints/Actors/Projectile/EnemyProjectile/BP_EnemyProjectile_Fast.BP_EnemyProjectile_Fast_C" (`KismetMathLibrary.MakeTransform` (`self.K2_GetActorLocation`)) "AlwaysSpawn" "MultiplyWithRoot" null null))
        (`KismetArrayLibrary.Array_Add` (`self.EnemyProjectilePool_Fast`) _returnvalue_2)))
    (:`CastFailed`
      (`KismetSystemLibrary.PrintString` "EnemyProjectileManager 게임모드 세팅 실패" true true (struct :`R` 1.0 :`A` 1.0) 5.0))))

(fn `ReturnProjectileToPool`
  (params (InProjectile :type "/Game/Blueprints/Actors/Projectile/BP_ProjectileBase Object Reference") (InType :type "/Game/Blueprints/Data/ProjectileData/E_EnemyProjectileType Enum" :default "NewEnumerator0"))
  (bind _enemyprojectilepool_normal (`self.EnemyProjectilePool_Normal`))
  (switch `/Game/Blueprints/Data/ProjectileData/E_EnemyProjectileType` InType
    (:`NewEnumerator0`
      (`KismetArrayLibrary.Array_Add` _enemyprojectilepool_normal InProjectile)
      (`KismetSystemLibrary.PrintString` (`KismetStringLibrary.Conv_IntToString` (`KismetArrayLibrary.Array_Length` _enemyprojectilepool_normal))))
    (:`NewEnumerator1`
      (`KismetArrayLibrary.Array_Add` (`self.EnemyProjectilePool_Fast`) InProjectile))))

(fn `SpawnFast`
  (params (MuzzleLocation :type "Vector Structure") (MuzzleRotation :type "Rotator Structure"))
  (bind _enemyprojectilepool_fast (`self.EnemyProjectilePool_Fast`))
  (bind _enemyprojectilepool_fast_2 (`self.EnemyProjectilePool_Fast`))
  (if (> (`KismetArrayLibrary.Array_Length` (`self.EnemyProjectilePool_Fast`)) 0)
    (`/Game/Blueprints/BPI_Poolable.OnActivate` (`|GetArrayItem` _enemyprojectilepool_fast_2 (`KismetArrayLibrary.Array_LastIndex` _enemyprojectilepool_fast_2)) MuzzleLocation MuzzleRotation)
    (`KismetArrayLibrary.Array_Remove` _enemyprojectilepool_fast (`KismetArrayLibrary.Array_LastIndex` _enemyprojectilepool_fast))))

(fn `SpawnNormal`
  (params (MuzzleLocation :type "Vector Structure") (MuzzleRotation :type "Rotator Structure"))
  (bind _enemyprojectilepool_normal (`self.EnemyProjectilePool_Normal`))
  (bind _enemyprojectilepool_normal_2 (`self.EnemyProjectilePool_Normal`))
  (if (> (`KismetArrayLibrary.Array_Length` (`self.EnemyProjectilePool_Normal`)) 0)
    (`/Game/Blueprints/BPI_Poolable.OnActivate` (`|GetArrayItem` _enemyprojectilepool_normal_2 (`KismetArrayLibrary.Array_LastIndex` _enemyprojectilepool_normal_2)) MuzzleLocation MuzzleRotation)
    (`KismetArrayLibrary.Array_Remove` _enemyprojectilepool_normal (`KismetArrayLibrary.Array_LastIndex` _enemyprojectilepool_normal))))

(fn `SpawnProjectileFromPool`
  (params (MuzzleLocation :type "Vector Structure") (MuzzleRotation :type "Rotator Structure") (NewParam :type "/Game/Blueprints/Data/ProjectileData/E_EnemyProjectileType Enum" :default "NewEnumerator0"))
  (switch `/Game/Blueprints/Data/ProjectileData/E_EnemyProjectileType` NewParam
    (:`NewEnumerator0`
      (`self.SpawnNormal` MuzzleLocation MuzzleRotation))
    (:`NewEnumerator1`
      (`self.SpawnFast` MuzzleLocation MuzzleRotation))))

(fn `UserConstructionScript`)
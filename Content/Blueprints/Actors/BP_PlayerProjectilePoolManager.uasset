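; Object pool manager for the player's Pierce, Normal and Grenade projectiles in the LineDefence game mode.
; On BeginPlay it registers itself on GM_LineDefence and pre-spawns up to MaxPoolSize actors of each type into separate arrays at its location.
; SpawnProjectileFromPool activates and removes the last entry of the requested pool, printing a message when empty.
; ReturnProjectileToPool adds a projectile back to the array matching its type.
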(event `self.ReceiveBeginPlay`
  ; 게임모드에 PlayerProjectileManager 저장
  (bind _asgm_line_defence (cast `/Game/Blueprints/Framework/GameMode/GM_LineDefence` (`GameplayStatics.GetGameMode`))
    (:`then`
      (set `/Game/Blueprints/Framework/GameMode/GM_LineDefence.PlayerProjectilePoolManager` self _asgm_line_defence)
      (for _ (range 1 (+ (`self.MaxPoolSize`) 1))
        (bind _returnvalue (`|SpawnActorFromClass` "/Game/Blueprints/Actors/Projectile/PlayerProjectile/BP_PlayerProjectile_Pierce.BP_PlayerProjectile_Pierce_C" (`KismetMathLibrary.MakeTransform` (`self.K2_GetActorLocation`)) "AlwaysSpawn" "MultiplyWithRoot" null null))
        (`KismetArrayLibrary.Array_Add` (`self.PlayerPiercePool`) _returnvalue)
        (bind _returnvalue_2 (`|SpawnActorFromClass` "/Game/Blueprints/Actors/Projectile/PlayerProjectile/BP_PlayerProjectile_Normal.BP_PlayerProjectile_Normal_C" (`KismetMathLibrary.MakeTransform` (`self.K2_GetActorLocation`)) "AlwaysSpawn" "MultiplyWithRoot" null null))
        (`KismetArrayLibrary.Array_Add` (`self.PlayerNormalPool`) _returnvalue_2)
        (bind _returnvalue_3 (`|SpawnActorFromClass` "/Game/Blueprints/Actors/Projectile/PlayerProjectile/BP_PlayerProjectile_Grenade.BP_PlayerProjectile_Grenade_C" (`KismetMathLibrary.MakeTransform` (`self.K2_GetActorLocation`)) "AlwaysSpawn" "MultiplyWithRoot" null null))
        (`KismetArrayLibrary.Array_Add` (`self.PlayerGrenadelPool`) _returnvalue_3)))
    (:`CastFailed`
      (`KismetSystemLibrary.PrintString` "PlayerProjectilePoolManager 게임모드 세팅 X" true true (struct :`R` 1.0 :`A` 1.0) 5.0))))

(fn `ReturnProjectileToPool`
  (params (InProjectile :type "/Game/Blueprints/Actors/Projectile/BP_ProjectileBase Object Reference") (InType :type "/Game/Blueprints/Data/ProjectileData/E_PlayerProjectileType Enum" :default "NewEnumerator0"))
  (switch `/Game/Blueprints/Data/ProjectileData/E_PlayerProjectileType` InType
    (:`NewEnumerator0`
      (`KismetArrayLibrary.Array_Add` (`self.PlayerPiercePool`) InProjectile))
    (:`NewEnumerator1`
      (`KismetArrayLibrary.Array_Add` (`self.PlayerNormalPool`) InProjectile))
    (:`NewEnumerator2`
      (`KismetArrayLibrary.Array_Add` (`self.PlayerGrenadelPool`) InProjectile))))

(fn `SpawnGrenade`
  (params (MuzzleLocation :type "Vector Structure") (MuzzleRotation :type "Rotator Structure"))
  (bind _playergrenadelpool (`self.PlayerGrenadelPool`))
  (bind _playergrenadelpool_2 (`self.PlayerGrenadelPool`))
  (if (> (`KismetArrayLibrary.Array_Length` (`self.PlayerGrenadelPool`)) 0)
    (`/Game/Blueprints/BPI_Poolable.OnActivate` :`self` (`|GetArrayItem` _playergrenadelpool (`KismetArrayLibrary.Array_LastIndex` _playergrenadelpool)) :`InLocation` MuzzleLocation :`InRotation` MuzzleRotation)
    (`KismetArrayLibrary.Array_Remove` _playergrenadelpool_2 (`KismetArrayLibrary.Array_LastIndex` _playergrenadelpool_2))
    (else
      ; PoolSize 체크
      (`KismetSystemLibrary.PrintString` "노말탄 pool empty" true true (struct :`R` 1.0 :`A` 1.0) 5.0))))

(fn `SpawnNormal`
  (params (MuzzleLocation :type "Vector Structure") (MuzzleRotation :type "Rotator Structure"))
  (bind _playernormalpool (`self.PlayerNormalPool`))
  (bind _playernormalpool_2 (`self.PlayerNormalPool`))
  (if (> (`KismetArrayLibrary.Array_Length` (`self.PlayerNormalPool`)) 0)
    (`/Game/Blueprints/BPI_Poolable.OnActivate` :`self` (`|GetArrayItem` _playernormalpool_2 (`KismetArrayLibrary.Array_LastIndex` _playernormalpool_2)) :`InLocation` MuzzleLocation :`InRotation` MuzzleRotation)
    (`KismetArrayLibrary.Array_Remove` _playernormalpool (`KismetArrayLibrary.Array_LastIndex` _playernormalpool))
    (else
      ; PoolSize 체크
      (`KismetSystemLibrary.PrintString` "노말탄 pool empty" true true (struct :`R` 1.0 :`A` 1.0) 5.0))))

(fn `SpawnPierce`
  (params (MuzzleLocation :type "Vector Structure") (MuzzleRotation :type "Rotator Structure"))
  (bind _playerpiercepool (`self.PlayerPiercePool`))
  (bind _playerpiercepool_2 (`self.PlayerPiercePool`))
  (if (> (`KismetArrayLibrary.Array_Length` (`self.PlayerPiercePool`)) 0)
    (`/Game/Blueprints/BPI_Poolable.OnActivate` :`self` (`|GetArrayItem` _playerpiercepool_2 (`KismetArrayLibrary.Array_LastIndex` _playerpiercepool_2)) :`InLocation` MuzzleLocation :`InRotation` MuzzleRotation)
    (`KismetArrayLibrary.Array_Remove` _playerpiercepool (`KismetArrayLibrary.Array_LastIndex` _playerpiercepool))
    (else
      ; PoolSize 체크
      (`KismetSystemLibrary.PrintString` "관통탄 pool empty" true true (struct :`R` 1.0 :`A` 1.0) 5.0))))

(fn `SpawnProjectileFromPool`
  (params (MuzzleLocation :type "Vector Structure") (MuzzleRotation :type "Rotator Structure") (NewParam :type "/Game/Blueprints/Data/ProjectileData/E_PlayerProjectileType Enum" :default "NewEnumerator0"))
  (switch `/Game/Blueprints/Data/ProjectileData/E_PlayerProjectileType` NewParam
    (:`NewEnumerator0`
      (`self.SpawnPierce` MuzzleLocation MuzzleRotation))
    (:`NewEnumerator1`
      (`self.SpawnNormal` MuzzleLocation MuzzleRotation))
    (:`NewEnumerator2`
      (`self.SpawnGrenade` MuzzleLocation MuzzleRotation))))

(fn `UserConstructionScript`)
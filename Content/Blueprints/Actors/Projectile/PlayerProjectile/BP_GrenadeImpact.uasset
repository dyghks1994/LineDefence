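; Grenade impact actor for the player's projectile that deals periodic area damage to enemies for a limited lifetime.
; On BeginPlay it sets the damage, plays a gunshot sound, applies the first hit immediately and starts a looping timer for later ticks.
; Each hit polls the sphere collision for overlapping BP_EnemyBase actors and sends OnHitMessage through BPI_HasHp.
; After LifeTime elapses it clears the timer and destroys itself.
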(event `self.ReceiveBeginPlay`
  (set `self.DamageAmount` 50)
  (`GameplayStatics.PlaySoundAtLocation` "/Game/_ExternalAsset/MEGA_FULL_BUNDLE/HIGH_TECH_WEAPON_SOUNDS/GUNSHOTS/WAVES/heavy_gunshot_v10.heavy_gunshot_v10" (`self.K2_GetActorLocation`) (struct) 1.0 1.0 0.0 null null null null)
  ; 1타는 즉시 적용하고 이후 interval 만큼 딜레이 적용
  (`self.ApplyPeriodicDamage`)
  (bind _returnvalue (`KismetSystemLibrary.K2_SetTimerDelegate` (`|CreateDelegate` :!event `ApplyPeriodicDamage`) (`self.DamageInterval`) true))
  (set `self.TImerHandle` _returnvalue)
  (`KismetSystemLibrary.Delay` (`self.LifeTime`))
  (`KismetSystemLibrary.K2_ClearAndInvalidateTimerHandle` (`self.TImerHandle`))
  (`self.K2_DestroyActor`))

(event `ApplyPeriodicDamage`
  (for _array_element (`PrimitiveComponent.GetOverlappingActors` (`self.SphereCollision`) "/Game/Blueprints/Actors/Character/Enemy/BP_EnemyBase.BP_EnemyBase_C")
    (if (`KismetSystemLibrary.DoesImplementInterface` _array_element "/Game/Blueprints/BPI_HasHp.BPI_HasHp_C")
      (message `/Game/Blueprints/BPI_HasHp.OnHit` _array_element (`self.DamageAmount`)))))

(fn `UserConstructionScript`)
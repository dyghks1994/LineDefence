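; Player projectile Blueprint for the Normal type, a child of a projectile parent that supplies its pool-return logic.
; BeginPlay sets its projectile type and base damage.
; On sphere overlap with an actor implementing BPI_HasHp, it sends that damage as a hit message, spawns a scaled, auto-released NS_Arrow_Cast Niagara effect and returns itself to the pool.
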(event `self.ReceiveBeginPlay`
  (`parent.ReceiveBeginPlay`)
  (set `self.PlayerProjectileType` "NewEnumerator1")
  (set `self.BaseDamage` 130))

(event `self.SphereCollision.OnComponentBeginOverlap`
  (params (OverlappedComponent :type "PrimitiveComponent Object Reference") (OtherActor :type "Actor Object Reference") (OtherComp :type "PrimitiveComponent Object Reference") (OtherBodyIndex :type Integer) (bFromSweep :type Boolean) (SweepResult :type "HitResult Structure (by ref)"))
  (if (`KismetSystemLibrary.DoesImplementInterface` OtherActor "/Game/Blueprints/BPI_HasHp.BPI_HasHp_C")
    (message `/Game/Blueprints/BPI_HasHp.OnHit` OtherActor (`self.BaseDamage`))
    ; 히트 이펙트
    (bind _returnvalue (`NiagaraFunctionLibrary.SpawnSystemAtLocation` "/Game/_ExternalAsset/Vefects/Anime_Stylized_VFX/VFX/Particles/NS_Arrow_Cast.NS_Arrow_Cast" (`self.K2_GetActorLocation`) (struct) (1.0 1.0 1.0) true true "AutoRelease"))
    (`NiagaraComponent.SetVariableFloat` _returnvalue "Scale Overall" 0.5)
    (`/Game/Blueprints/BPI_Poolable.ReturnToPool`)))

(fn `UserConstructionScript`
  (`parent.UserConstructionScript`))
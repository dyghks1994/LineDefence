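; BP_PlayerProjectile_Grenade is a pooled player projectile that explodes by spawning a BP_GrenadeImpact actor and returning to its pool.
; It sets its projectile type and base damage on BeginPlay, then randomizes a short flight time on each activation.
; Tick triggers the explosion when that time runs out or the grenade crosses the side Y bounds.
; Overlapping an actor that implements BPI_HasHp also detonates it.
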(event `self.ReceiveBeginPlay`
  (`parent.ReceiveBeginPlay`)
  (set `self.PlayerProjectileType` "NewEnumerator2")
  (set `self.BaseDamage` 50))

(event `self.ReceiveTick`
  (params (DeltaSeconds :type "Float (single-precision)"))
  (bind (_returnvalue_x _returnvalue_y) (`KismetMathLibrary.BreakVector` (`self.K2_GetActorLocation`)))
  (`parent.ReceiveTick` DeltaSeconds)
  ; 이동시간 검사
  (bind _output_get (set `self.MoveDuration` (- (`self.MoveDuration`) DeltaSeconds)))
  (if (or (<= _output_get 0.0) (or (< _returnvalue_y -350.0) (> _returnvalue_y 350.0)))
    (`self.SpawnGrenadeImpact`)
    (`/Game/Blueprints/BPI_Poolable.ReturnToPool`)))

(event `/Game/Blueprints/BPI_Poolable.OnActivate`
  (params (InLocation :type "Vector Structure") (InRotation :type "Rotator Structure") (InStat :type "/Game/Blueprints/Data/SpawnData/ST_EnemyStat Structure"))
  (`parent.OnActivate` InLocation InRotation (struct))
  ; 이동 시간 랜덤 보정
  (set `self.MoveDuration` (`KismetMathLibrary.RandomFloatInRange` 0.8 1.0)))

(event `self.SphereCollision.OnComponentBeginOverlap`
  (params (OverlappedComponent :type "PrimitiveComponent Object Reference") (OtherActor :type "Actor Object Reference") (OtherComp :type "PrimitiveComponent Object Reference") (OtherBodyIndex :type Integer) (bFromSweep :type Boolean) (SweepResult :type "HitResult Structure (by ref)"))
  (if (`KismetSystemLibrary.DoesImplementInterface` OtherActor "/Game/Blueprints/BPI_HasHp.BPI_HasHp_C")
    (`self.SpawnGrenadeImpact`)
    (`/Game/Blueprints/BPI_Poolable.ReturnToPool`)))

(fn `SpawnGrenadeImpact`
  (`|SpawnActorFromClass` "/Game/Blueprints/Actors/Projectile/PlayerProjectile/BP_GrenadeImpact.BP_GrenadeImpact_C" (`KismetMathLibrary.MakeTransform` (`self.K2_GetActorLocation`)) "AlwaysSpawn" "MultiplyWithRoot" null null))

(fn `UserConstructionScript`
  (`parent.UserConstructionScript`))
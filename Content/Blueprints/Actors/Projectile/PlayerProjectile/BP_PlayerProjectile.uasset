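; BP_PlayerProjectile is a pooled player projectile for the line defence game mode.
; On BeginPlay it caches the projectile pool manager from GM_LineDefence.
; When its collision sphere overlaps a BP_EnemyBase actor, it spawns a half-scale, auto-released Niagara effect and returns to the pool.
; Returning runs the parent deactivation, then hands the projectile back to the manager under its projectile type.
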(event `self.ReceiveBeginPlay`
  (`parent.ReceiveBeginPlay`)
  (bind _asgm_line_defence (cast `/Game/Blueprints/Framework/GameMode/GM_LineDefence` (`GameplayStatics.GetGameMode`)))
  (set `self.PlayerProjectilePoolManager` (`/Game/Blueprints/Framework/GameMode/GM_LineDefence.PlayerProjectilePoolManager` _asgm_line_defence)))

(event `/Game/Blueprints/BPI_Poolable.OnDeactivate`
  (`parent.OnDeactivate`))

(event `/Game/Blueprints/BPI_Poolable.ReturnToPool`
  (bind _playerprojectilepoolmanager (`self.PlayerProjectilePoolManager`))
  (`/Game/Blueprints/BPI_Poolable.OnDeactivate`)
  ; SpawnPoolManager에 다시 추가
  (`/Engine/EditorBlueprintResources/StandardMacros.IsValid` _playerprojectilepoolmanager
    (:`Is Valid`
      (`/Game/Blueprints/Actors/BP_PlayerProjectilePoolManager.ReturnProjectileToPool` _playerprojectilepoolmanager self (`self.PlayerProjectileType`)))))

(event `self.SphereCollision.OnComponentBeginOverlap`
  (params (OverlappedComponent :type "PrimitiveComponent Object Reference") (OtherActor :type "Actor Object Reference") (OtherComp :type "PrimitiveComponent Object Reference") (OtherBodyIndex :type Integer) (bFromSweep :type Boolean) (SweepResult :type "HitResult Structure (by ref)"))
  (if (`KismetMathLibrary.ClassIsChildOf` (`GameplayStatics.GetObjectClass` OtherActor) "/Game/Blueprints/Actors/Character/Enemy/BP_EnemyBase.BP_EnemyBase_C")
    (bind _returnvalue (`NiagaraFunctionLibrary.SpawnSystemAtLocation` "/Game/_ExternalAsset/Vefects/Anime_Stylized_VFX/VFX/Particles/NS_Arrow_Cast.NS_Arrow_Cast" (`self.K2_GetActorLocation`) (struct) (1.0 1.0 1.0) true true "AutoRelease"))
    (`NiagaraComponent.SetVariableFloat` _returnvalue "Scale Overall" 0.5)
    (`/Game/Blueprints/BPI_Poolable.ReturnToPool`)))

(fn `GetAsActor`
  (returns (OutActor :type "Actor Object Reference"))
  (return null))

(fn `UserConstructionScript`
  (`parent.UserConstructionScript`))
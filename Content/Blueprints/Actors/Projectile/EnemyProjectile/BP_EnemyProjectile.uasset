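; Pooled enemy projectile for the line-defence mode that damages the defence line on contact.
; BeginPlay caches the enemy projectile pool manager from GM_LineDefence.
; Any sphere overlap deactivates it and returns it to the pool by projectile type.
; If the overlapped actor is a BP_DefenceLine, it sends base damage through the BPI_HasHp hit message; otherwise it prints the actor's name.
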(event `self.ReceiveBeginPlay`
  (`parent.ReceiveBeginPlay`)
  ; 에너미 풀 세팅
  (bind _asgm_line_defence (cast `/Game/Blueprints/Framework/GameMode/GM_LineDefence` (`GameplayStatics.GetGameMode`)))
  (set `self.EnemyProjectilePoolManager` (`/Game/Blueprints/Framework/GameMode/GM_LineDefence.EnemyProjectilePoolManager` _asgm_line_defence)))

(event `/Game/Blueprints/BPI_Poolable.ReturnToPool`
  (bind _enemyprojectilepoolmanager (`self.EnemyProjectilePoolManager`))
  (`/Game/Blueprints/BPI_Poolable.OnDeactivate`)
  ; SpawnPoolManager에 다시 추가
  (`/Engine/EditorBlueprintResources/StandardMacros.IsValid` _enemyprojectilepoolmanager
    (:`Is Valid`
      (`/Game/Blueprints/Actors/BP_EnemyProjectilePoolManager.ReturnProjectileToPool` _enemyprojectilepoolmanager self (`self.EnemyProjectileType`)))))

(event `self.SphereCollision.OnComponentBeginOverlap`
  (params (OverlappedComponent :type "PrimitiveComponent Object Reference") (OtherActor :type "Actor Object Reference") (OtherComp :type "PrimitiveComponent Object Reference") (OtherBodyIndex :type Integer) (bFromSweep :type Boolean) (SweepResult :type "HitResult Structure (by ref)"))
  (`/Game/Blueprints/BPI_Poolable.ReturnToPool`)
  (if (`KismetMathLibrary.ClassIsChildOf` (`GameplayStatics.GetObjectClass` OtherActor) "/Game/Blueprints/Actors/Wall/BP_DefenceLine.BP_DefenceLine_C")
    (if (`KismetSystemLibrary.DoesImplementInterface` OtherActor "/Game/Blueprints/BPI_HasHp.BPI_HasHp_C")
      (message `/Game/Blueprints/BPI_HasHp.OnHit` OtherActor (`self.BaseDamage`)))
    (else
      (`KismetSystemLibrary.PrintString` (`KismetSystemLibrary.GetDisplayName` OtherActor)))))

(fn `UserConstructionScript`
  (`parent.UserConstructionScript`))
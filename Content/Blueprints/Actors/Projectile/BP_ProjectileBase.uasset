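; Base projectile actor built for reuse through an object pool, starting hidden and inactive on BeginPlay.
; OnActivate enables rendering, tick and collision, places it at the given location and yaw, launches it along local X via ProjectileMovement and starts a lifetime timer.
; OnDeactivate disables rendering, tick and collision without stopping movement.
; Pool accessors return self and a zero location; overlap has no hit logic.
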(event `self.ReceiveBeginPlay`
  (`/Game/Blueprints/BPI_Poolable.OnDeactivate`))

(event `/Game/Blueprints/BPI_Poolable.OnActivate`
  (params (InLocation :type "Vector Structure") (InRotation :type "Rotator Structure") (InStat :type "/Game/Blueprints/Data/SpawnData/ST_EnemyStat Structure"))
  ; ObjectPool에서 스폰할 때 활성화
  ;; 렌더, 틱, 충돌 설정
  (`self.SetActorHiddenInGame` false)
  (`self.SetActorTickEnabled` true)
  (`self.SetActorEnableCollision` true)
  ;; 스폰위치, 방향 설정
  (`MovementComponent.StopMovementImmediately` (`self.ProjectileMovement`))
  (`self.K2_SetActorLocationAndRotation` InLocation (`KismetMathLibrary.MakeRotator` 0.0 0.0 (.yaw InRotation)))
  (`ProjectileMovementComponent.SetVelocityInLocalSpace` (`self.ProjectileMovement`) (`KismetMathLibrary.MakeVector` (`self.MoveSpeed`)))
  ;; 발사체 유지시간 설정
  (bind _returnvalue (`KismetSystemLibrary.K2_SetTimerDelegate` (`|CreateDelegate` :!event `ReturnToPool`) (`self.LifeTIme`)))
  (set `self.LifeTImerHandle` _returnvalue)
  ;; 데미지 설정
  (set `self.BaseDamage` (`self.BaseDamage`)))

(event `/Game/Blueprints/BPI_Poolable.OnDeactivate`
  ; 비활성화(렌더, 충돌, 이동 멈춤)
  (`self.SetActorHiddenInGame` true)
  (`self.SetActorTickEnabled` false)
  (`self.SetActorEnableCollision` false))

(fn `GetAsActor`
  (returns (OutActor :type "Actor Object Reference"))
  (return self))

(fn `GetPoolableLocation`
  (returns (OutLocation :type "Vector Structure"))
  (return (0.0 0.0 0.0)))

(fn `UserConstructionScript`)
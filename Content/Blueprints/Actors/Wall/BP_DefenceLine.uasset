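; BP_DefenceLine is the defence wall actor whose life reaching zero signals game over.
; OnHit and Heal adjust clamped life, with Heal adding a fraction of max, and broadcast percent and ratio through OnChangedLife.
; Surviving hits play a timeline driving FlashAmount on the wall's dynamic material.
; At zero life it registers with GM_LineDefence if no line is set, binding game over just before broadcasting OnGameOver.
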(event `self.ReceiveBeginPlay`
  (bind _asgm_line_defence (cast `/Game/Blueprints/Framework/GameMode/GM_LineDefence` (`GameplayStatics.GetGameMode`))
    (:`then`
      (set `self.GM_LineDefence` _asgm_line_defence))
    (:`CastFailed`
      _))
  (bind _returnvalue (`KismetMaterialLibrary.CreateDynamicMaterialInstance` "/Game/_ExternalAsset/TreatmentStation/Materials/MaterialInstance/MI_Trim_Panel_2.MI_Trim_Panel_2"))
  (bind _output_get (set `self.MID` _returnvalue))
  (`PrimitiveComponent.SetMaterial` (`self.WallMesh`) 1 _output_get)
  (set `self.CurrentLife` (`self.MaxLife`)))

(event `self.BoxCollision.OnComponentBeginOverlap`
  (params (OverlappedComponent :type "PrimitiveComponent Object Reference") (OtherActor :type "Actor Object Reference") (OtherComp :type "PrimitiveComponent Object Reference") (OtherBodyIndex :type Integer) (bFromSweep :type Boolean) (SweepResult :type "HitResult Structure (by ref)")))

(event `/Game/Blueprints/BPI_HasHp.OnHit`
  (params (InDamage :type Integer))
  (bind _gm_linedefence (`self.GM_LineDefence`))
  (set `self.CurrentLife` (`KismetMathLibrary.Max` (- (`self.CurrentLife`) InDamage)))
  (`self.UpdateLife`)
  (if (<= (`self.CurrentLife`) 0)
    ; 플레이어 생성이 게임모드보다 느려서 플레이어 쪽에서 첫 레벨업 때 게임모드의 이벤트 바인딩 호출
    (`/Engine/EditorBlueprintResources/StandardMacros.IsValid` _gm_linedefence
      (:`Is Valid`
        (`/Engine/EditorBlueprintResources/StandardMacros.IsValid` (`/Game/Blueprints/Framework/GameMode/GM_LineDefence.DefenceLine` _gm_linedefence)
          (:`Is Valid`
            _)
          (:`Is Not Valid`
            (set `/Game/Blueprints/Framework/GameMode/GM_LineDefence.DefenceLine` self _gm_linedefence)
            (`/Game/Blueprints/Framework/GameMode/GM_LineDefence.BindEventGameOver` _gm_linedefence)))
        (`self.OnGameOver`)))
    (else
      (bind (_direction _value) (`Timeline|TL_Flash` :!via `PlayFromStart`)
        (:`Update`
          (`MaterialInstanceDynamic.SetScalarParameterValue` (`self.MID`) "FlashAmount" _value))))))

(event `/Game/Blueprints/BPI_HasHp.Heal`
  (params (HealPercent :type "Float (double-precision)"))
  (set `self.CurrentLife` (`KismetMathLibrary.FTrunc` (`KismetMathLibrary.FClamp` (+ (* HealPercent (`KismetMathLibrary.Conv_IntToDouble` (`self.MaxLife`))) (`KismetMathLibrary.Conv_IntToDouble` (`self.CurrentLife`))) 0.0 (`KismetMathLibrary.Conv_IntToDouble` (`self.MaxLife`)))))
  (`self.UpdateLife`))

(fn `UpdateLife`
  (bind _returnvalue (/ (`KismetMathLibrary.Conv_IntToDouble` (`self.CurrentLife`)) (`KismetMathLibrary.Conv_IntToDouble` (`self.MaxLife`))))
  (`self.OnChangedLife` (`KismetMathLibrary.Conv_Int64ToDouble` (`KismetMathLibrary.FTrunc64` (* _returnvalue 100.0))) _returnvalue))

(fn `UserConstructionScript`)
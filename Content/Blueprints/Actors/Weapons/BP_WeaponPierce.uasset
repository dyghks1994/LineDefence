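; BP_WeaponPierce is a player weapon Blueprint that fires pooled projectiles at its target actor.
; On fire, it spawns a projectile from PlayerProjectilePoolManager at the muzzle's XY and a fixed height, aimed only in the horizontal plane toward the target's poolable location.
; It then restarts the fire montage on the player's anim instance, first setting up the mesh and anim references if the mesh is invalid.
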(event `self.OnFire`
  (bind _playeraniminstance (`self.PlayerAnimInstance`))
  (bind _animmfire (`self.AnimmFire`))
  (bind _targetactor (`self.TargetActor`))
  (bind (_returnvalue_x _returnvalue_y) (`KismetMathLibrary.BreakVector` (`SceneComponent.K2_GetComponentLocation` (`self.Muzzle`))))
  (bind (_returnvalue_x_2 _returnvalue_y_2 _returnvalue_z) (`KismetMathLibrary.BreakVector` (`SceneComponent.K2_GetComponentLocation` (`self.Muzzle`))))
  ; z축값 차이는 제외하고 x,y 방향만 계산
  (`/Engine/EditorBlueprintResources/StandardMacros.IsValid` (`KismetSystemLibrary.Conv_InterfaceToObject` _targetactor)
    (:`Is Valid`
      (bind _outlocation (`/Game/Blueprints/BPI_Poolable.GetPoolableLocation` _targetactor))
      (`/Game/Blueprints/Actors/BP_PlayerProjectilePoolManager.SpawnProjectileFromPool` (`self.PlayerProjectilePoolManager`) (`KismetMathLibrary.MakeVector` _returnvalue_x _returnvalue_y 30.0) (`KismetMathLibrary.FindLookAtRotation` (`KismetMathLibrary.MakeVector` _returnvalue_x_2 _returnvalue_y_2 _returnvalue_z) (`KismetMathLibrary.MakeVector` (.x _outlocation) (.y _outlocation) _returnvalue_z)) "NewEnumerator0")
      ; 사격 애니메이션 재생
      (`/Engine/EditorBlueprintResources/StandardMacros.IsValid` (`self.PlayerSkeletalMesh`)
        (:`Is Valid`
          _)
        (:`Is Not Valid`
          (`self.SetPlayerSkeletalMeshAndAnimInstace`)))
      (`AnimInstance.Montage_Stop` _playeraniminstance 0.0 _animmfire)
      (`AnimInstance.Montage_Play` _playeraniminstance _animmfire 2.0 "MontageLength" 0.0 false))))

(event `TriggerSpawnProjectile`)

(fn `UserConstructionScript`
  (`parent.UserConstructionScript`))
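; Enemy pool manager for the line defence game mode that pre-spawns melee and ranged enemies and runs their waves.
; StartWave queues that wave's DataTable rows with scaled stats, and a looping timer releases the head once elapsed time reaches its WaveCount (not SpawnTime).
; Spawns activate pooled enemies at random Y between side markers.
; Returned enemies rejoin their pool, changing game state when queue and active list are empty.
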(event `self.ReceiveBeginPlay`
  ; 게임모드에 EnemyPoolManager 저장
  (bind _asgm_line_defence (cast `/Game/Blueprints/Framework/GameMode/GM_LineDefence` (`GameplayStatics.GetGameMode`))
    (:`then`
      (set `self.GM_LineDefence` _asgm_line_defence)
      (set `/Game/Blueprints/Framework/GameMode/GM_LineDefence.EnemyPoolManager` self _asgm_line_defence)
      ; 오프젝트 풀 초기화
      (for _ (range 1 (+ (`self.MaxPoolSize`) 1))
        (bind _returnvalue (`|SpawnActorFromClass` "/Game/Blueprints/Actors/Character/Enemy/BP_EnemyMelee.BP_EnemyMelee_C" (`KismetMathLibrary.MakeTransform` (`self.K2_GetActorLocation`)) "AlwaysSpawn" "MultiplyWithRoot" null null))
        (`KismetArrayLibrary.Array_Add` (`self.NormalEnemyPool`) _returnvalue)
        (bind _returnvalue_2 (`|SpawnActorFromClass` "/Game/Blueprints/Actors/Character/Enemy/BP_EnemyRanged.BP_EnemyRanged_C" (`KismetMathLibrary.MakeTransform` (`self.K2_GetActorLocation`)) "AlwaysSpawn" "MultiplyWithRoot" null null))
        (`KismetArrayLibrary.Array_Add` (`self.FastEnemyPool`) _returnvalue_2))
      ; 스폰 데이터 초기화
      (`self.GetSpawnData`))
    (:`CastFailed`
      (`KismetSystemLibrary.PrintString` "EnemyPoolManager 게임모드 세팅 실패" true true (struct :`R` 1.0 :`A` 1.0)))))

(event `StartWave`
  (params (InWaveNum :type Integer))
  ; 이전 웨이브 큐 클리어
  (`KismetArrayLibrary.Array_Clear` (`self.SpawnQueue`))
  (for _array_element (`self.SpawnDataArray`)
    (bind (_wavecount _spawntime _enemytype _basehp _basespeed _statmultiplier) (break `/Game/Blueprints/Data/SpawnData/ST_SpawnRawData` _array_element))
    ; N번째 웨이브 데이터만 필터링해서 스폰 큐에 추가
    (if (== _wavecount InWaveNum)
      (`KismetArrayLibrary.Array_Add` (`self.SpawnQueue`) (make `/Game/Blueprints/Data/SpawnData/ST_SpawnQueueData` _wavecount _spawntime _enemytype (make `/Game/Blueprints/Data/SpawnData/ST_EnemyStat` _basehp _basespeed (* _wavecount _statmultiplier))))))
  (set `self.ElapsedTime` 0.0)
  (bind _returnvalue (`KismetSystemLibrary.K2_SetTimerDelegate` (`|CreateDelegate` :!event `CheckSpawnQueue`) (`self.SpawnQueueCheckTime`) true))
  (set `self.WaveTimerHandle` _returnvalue)
  (`KismetSystemLibrary.PrintString` (`KismetStringLibrary.BuildString_Int` "" "Wave" (`/Game/Blueprints/Framework/GameMode/GM_LineDefence.CurrentWaveNumber` (`self.GM_LineDefence`)) " 시작")))

(event `CheckSpawnQueue`
  (bind _spawnqueue (`self.SpawnQueue`))
  (bind (_wavecount _spawntime _enemytype _enemystat) (break `/Game/Blueprints/Data/SpawnData/ST_SpawnQueueData` (`|GetArrayItem` _spawnqueue)))
  ; 웨이브 타임 초기화
  (set `self.ElapsedTime` (+ (`self.ElapsedTime`) (`self.SpawnQueueCheckTime`)))
  (if (> (`KismetArrayLibrary.Array_Length` _spawnqueue) 0)
    ; 스폰 타이밍 체크
    (if (>= (`self.ElapsedTime`) _wavecount)
      (`self.SpawnEnemyFromPool` _enemytype _enemystat)
      (`KismetArrayLibrary.Array_Remove` _spawnqueue))
    (else
      (`KismetSystemLibrary.PrintString` (`KismetStringLibrary.BuildString_Int` "" "Wave" (`/Game/Blueprints/Framework/GameMode/GM_LineDefence.CurrentWaveNumber` (`self.GM_LineDefence`)) "스폰 끝"))
      (`KismetSystemLibrary.K2_ClearAndInvalidateTimerHandle` (`self.WaveTimerHandle`)))))

(fn `GetSpawnData`
  (bind _outrownames (`DataTableFunctionLibrary.GetDataTableRowNames` "/Game/Blueprints/Data/SpawnData/DT_SpawnRawData.DT_SpawnRawData"))
  (for _array_element _outrownames
    (bind _returnvalue (`|GetDataTableRow` "/Game/Blueprints/Data/SpawnData/DT_SpawnRawData.DT_SpawnRawData" _array_element)
      (:`then`
        (`KismetArrayLibrary.Array_Add` (`self.SpawnDataArray`) _returnvalue))))
  (`KismetSystemLibrary.PrintString` "스폰데이터 초기화"))

(fn `IsWaveClear`
  (returns (OutIsClear :type Boolean))
  (bind _returnvalue (`KismetArrayLibrary.Array_Length` (`self.ActiveEnemies`)))
  (bind _returnvalue_2 (and (== _returnvalue 0) (== (`KismetArrayLibrary.Array_Length` (`self.SpawnQueue`)) 0)))
  ; Wave 클리어 판별
  (if _returnvalue_2
    (`KismetSystemLibrary.PrintString` "Wave 클리어" true true (struct :`R` 0.63921 :`B` 1.0 :`A` 1.0))
    (return _returnvalue_2)
    (else
      (`KismetSystemLibrary.PrintString` (`KismetStringLibrary.BuildString_Int` "" "남은 적 :" _returnvalue "마리") true true (struct :`R` 0.63921 :`B` 1.0 :`A` 1.0)))))

(fn `ReturnEnemyToPool`
  (params (InEnemy :type "/Game/Blueprints/Actors/Character/Enemy/BP_EnemyBase Object Reference") (InType :type "/Game/Blueprints/Data/SpawnData/E_EnemyType Enum" :default "NewEnumerator0"))
  (bind _activeenemies (`self.ActiveEnemies`))
  ; 활성 풀에서 제거
  (if (`KismetArrayLibrary.Array_Contains` _activeenemies InEnemy)
    (bind _returnvalue (`KismetArrayLibrary.Array_RemoveItem` _activeenemies InEnemy))
    (if _returnvalue
      ; EnemyType별 Pool로 회수
      (switch `/Game/Blueprints/Data/SpawnData/E_EnemyType` InType
        (:`NewEnumerator0`
          (`KismetArrayLibrary.Array_Add` (`self.NormalEnemyPool`) InEnemy))
        (:`NewEnumerator1`
          (`KismetArrayLibrary.Array_Add` (`self.FastEnemyPool`) InEnemy)))
      ; 적 처치시 마다 wave 클리어 상태 체크
      (bind _outisclear (`self.IsWaveClear`))
      (if _outisclear
        (`/Game/Blueprints/Framework/GameMode/GM_LineDefence.SetGameState` (`self.GM_LineDefence`) "NewEnumerator2"))
      (else
        (`KismetSystemLibrary.PrintString` "ActivateEnemies 제거 실패" true true (struct :`R` 1.0 :`A` 1.0))))
    (else
      ; 중복 제거 방지 예외처리
      (`KismetSystemLibrary.PrintString` (`KismetStringLibrary.Concat_StrStr` (`KismetSystemLibrary.GetDisplayName` InEnemy) "이미 활성풀에서 제거 됨")))))

(fn `SpawnEnemy_Melee`
  (params (InStat :type "/Game/Blueprints/Data/SpawnData/ST_EnemyStat Structure"))
  (bind (_returnvalue_x _returnvalue_y _returnvalue_z) (`KismetMathLibrary.BreakVector` (`self.K2_GetActorLocation`)))
  (bind _normalenemypool (`self.NormalEnemyPool`))
  (bind _returnvalue (`KismetArrayLibrary.Array_LastIndex` _normalenemypool))
  (bind (_returnvalue_x_2 _returnvalue_y_2) (`KismetMathLibrary.BreakVector` (`self.K2_GetActorLocation` (`self.RightSide`))))
  (bind (_returnvalue_x_3 _returnvalue_y_3) (`KismetMathLibrary.BreakVector` (`self.K2_GetActorLocation` (`self.LeftSide`))))
  (bind _output (`|GetArrayItem` _normalenemypool _returnvalue))
  (if (> (`KismetArrayLibrary.Array_Length` (`self.NormalEnemyPool`)) 0)
    ; 스폰 후 활성화 Enemy 배열에 add해서 관리
    (`/Game/Blueprints/BPI_Poolable.OnActivate` :`self` _output :`InLocation` (`KismetMathLibrary.MakeVector` _returnvalue_x (`KismetMathLibrary.RandomFloatInRange` _returnvalue_y_3 _returnvalue_y_2) _returnvalue_z) :`InStat` InStat)
    (`KismetArrayLibrary.Array_Add` (`self.ActiveEnemies`) _output)
    ; SpawnPool에서 제거
    (`KismetArrayLibrary.Array_Remove` _normalenemypool _returnvalue)
    (else
      ; PoolSize 체크
      (`KismetSystemLibrary.PrintString` "EnemyPool 부족" true true (struct :`R` 1.0 :`A` 1.0)))))

(fn `SpawnEnemy_Ranged`
  (params (InStat :type "/Game/Blueprints/Data/SpawnData/ST_EnemyStat Structure"))
  (bind (_returnvalue_x _returnvalue_y _returnvalue_z) (`KismetMathLibrary.BreakVector` (`self.K2_GetActorLocation`)))
  (bind _fastenemypool (`self.FastEnemyPool`))
  (bind _returnvalue (`KismetArrayLibrary.Array_LastIndex` _fastenemypool))
  (bind (_returnvalue_x_2 _returnvalue_y_2) (`KismetMathLibrary.BreakVector` (`self.K2_GetActorLocation` (`self.RightSide`))))
  (bind (_returnvalue_x_3 _returnvalue_y_3) (`KismetMathLibrary.BreakVector` (`self.K2_GetActorLocation` (`self.LeftSide`))))
  (bind _output (`|GetArrayItem` _fastenemypool _returnvalue))
  (if (> (`KismetArrayLibrary.Array_Length` (`self.FastEnemyPool`)) 0)
    ; 스폰 후 활성화 Enemy 배열에 add해서 관리
    (`/Game/Blueprints/BPI_Poolable.OnActivate` :`self` _output :`InLocation` (`KismetMathLibrary.MakeVector` _returnvalue_x (`KismetMathLibrary.RandomFloatInRange` _returnvalue_y_3 _returnvalue_y_2) _returnvalue_z) :`InStat` InStat)
    (`KismetArrayLibrary.Array_Add` (`self.ActiveEnemies`) _output)
    ; SpawnPool에서 제거
    (`KismetArrayLibrary.Array_Remove` _fastenemypool _returnvalue)
    (else
      ; PoolSize 체크
      (`KismetSystemLibrary.PrintString` "EnemyPool 부족" true true (struct :`R` 1.0 :`A` 1.0)))))

(fn `SpawnEnemyFromPool`
  (params (InType :type "/Game/Blueprints/Data/SpawnData/E_EnemyType Enum" :default "NewEnumerator0") (InStat :type "/Game/Blueprints/Data/SpawnData/ST_EnemyStat Structure"))
  (switch `/Game/Blueprints/Data/SpawnData/E_EnemyType` InType
    (:`NewEnumerator0`
      (`self.SpawnEnemy_Melee` InStat))
    (:`NewEnumerator1`
      (`self.SpawnEnemy_Ranged` InStat))))

(fn `UserConstructionScript`)
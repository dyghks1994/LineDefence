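; Display actor that showcases Vefects explosion effects, pairing a Niagara system with a matching sound cue.
; The construction script picks both from the Location (Ground or Aerial) and Select type, and offsets the FX vertically for that location.
; Some types, such as Water, Thermite and Artillery, reuse their ground effect when aerial.
; BeginPlay and ReplayButton restart both components, then loop through a retriggerable delay of LoopDelayTime.
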(event `Replay Button`
  (`ActorComponent.Activate` (`self.SFX`) true :!label _label)
  (`ActorComponent.Activate` (`self.FX`) true)
  (`KismetSystemLibrary.RetriggerableDelay` (`self.LoopDelayTime`))
  (goto _label))

(event `self.ReceiveBeginPlay`
  (goto _label))

(fn `UserConstructionScript`
  (bind _fx (`self.FX`))
  (bind _fx_2 (`self.FX`))
  (bind _sfx (`self.SFX`))
  (bind _sfx_2 (`self.SFX`))
  (bind _fx_3 (`self.FX`))
  (switch `/Game/_ExternalAsset/Vefects/Explosions_VFX/Blueprints/BP_Enum_Explosion_Location` (`self.Location`)
    (:`NewEnumerator0`
      (`SceneComponent.K2_AddLocalOffset` _fx (0.0 0.0 3.0) false false)
      (switch `/Game/_ExternalAsset/Vefects/Explosions_VFX/Blueprints/BP_Enum_Explosion_Type` (`self.Select`)
        (:`NewEnumerator0`
          (`NiagaraComponent.SetAsset` _fx_3 "/Game/_ExternalAsset/Vefects/Explosions_VFX/VFX/Generic/BaseColors/NS_ExplosionGenericLarge_Once.NS_ExplosionGenericLarge_Once" true)
          (`AudioComponent.SetSound` _sfx_2 "/Game/_ExternalAsset/Vefects/Explosions_VFX/Audio/SFX_Vefects_Explosion_Generic_Cue.SFX_Vefects_Explosion_Generic_Cue"))
        (:`NewEnumerator1`
          (`NiagaraComponent.SetAsset` _fx_3 "/Game/_ExternalAsset/Vefects/Explosions_VFX/VFX/Grenade/NS_ExplosionGrenade_Once.NS_ExplosionGrenade_Once" true)
          (`AudioComponent.SetSound` _sfx_2 "/Game/_ExternalAsset/Vefects/Explosions_VFX/Audio/SFX_Vefects_Explosion_Grenade_Cue.SFX_Vefects_Explosion_Grenade_Cue"))
        (:`NewEnumerator2`
          (`NiagaraComponent.SetAsset` _fx_3 "/Game/_ExternalAsset/Vefects/Explosions_VFX/VFX/Molotov/NS_MolotovExplosion_Once.NS_MolotovExplosion_Once" true)
          (`AudioComponent.SetSound` _sfx_2 "/Game/_ExternalAsset/Vefects/Explosions_VFX/Audio/SFX_Vefects_Explosion_Incendiary_Cue.SFX_Vefects_Explosion_Incendiary_Cue"))
        (:`NewEnumerator3`
          (`NiagaraComponent.SetAsset` _fx_3 "/Game/_ExternalAsset/Vefects/Explosions_VFX/VFX/Generic/Toxic/NS_ExplosionGenericLarge_Toxic_Once.NS_ExplosionGenericLarge_Toxic_Once" true)
          (`AudioComponent.SetSound` _sfx_2 "/Game/_ExternalAsset/Vefects/Explosions_VFX/Audio/SFX_Vefects_Explosion_Hellfire_Cue.SFX_Vefects_Explosion_Hellfire_Cue"))
        (:`NewEnumerator4`
          (`NiagaraComponent.SetAsset` _fx_3 "/Game/_ExternalAsset/Vefects/Explosions_VFX/VFX/Generic/BlackBody/NS_ExplosionGenericLarge_Blackbody_Once.NS_ExplosionGenericLarge_Blackbody_Once" true)
          (`AudioComponent.SetSound` _sfx_2 "/Game/_ExternalAsset/Vefects/Explosions_VFX/Audio/SFX_Vefects_Explosion_Black_Cue.SFX_Vefects_Explosion_Black_Cue"))
        (:`NewEnumerator5`
          (`NiagaraComponent.SetAsset` _fx_3 "/Game/_ExternalAsset/Vefects/Explosions_VFX/VFX/Sci-Fi/NS_ElectricExplosion_Once.NS_ElectricExplosion_Once" true)
          (`AudioComponent.SetSound` _sfx_2 "/Game/_ExternalAsset/Vefects/Explosions_VFX/Audio/SFX_Vefects_Explosion_Electric_Cue.SFX_Vefects_Explosion_Electric_Cue"))
        (:`NewEnumerator6`
          (`NiagaraComponent.SetAsset` _fx_3 "/Game/_ExternalAsset/Vefects/Explosions_VFX/VFX/GasGrenade/NS_GasGrenade_Medium_Once.NS_GasGrenade_Medium_Once" true)
          (`AudioComponent.SetSound` _sfx_2 "/Game/_ExternalAsset/Vefects/Explosions_VFX/Audio/SFX_Vefects_Explosion_Gas_Cue.SFX_Vefects_Explosion_Gas_Cue"))
        (:`NewEnumerator7`
          (`NiagaraComponent.SetAsset` _fx_3 "/Game/_ExternalAsset/Vefects/Explosions_VFX/VFX/Water/NS_WaterExplosion_Once.NS_WaterExplosion_Once" true)
          (`AudioComponent.SetSound` _sfx_2 "/Game/_ExternalAsset/Vefects/Explosions_VFX/Audio/SFX_Vefects_Explosion_Water_Cue.SFX_Vefects_Explosion_Water_Cue"))
        (:`NewEnumerator8`
          (`NiagaraComponent.SetAsset` _fx_3 "/Game/_ExternalAsset/Vefects/Explosions_VFX/VFX/Thermite/NS_ThermiteGrenade_Once.NS_ThermiteGrenade_Once" true)
          (`AudioComponent.SetSound` _sfx_2 "/Game/_ExternalAsset/Vefects/Explosions_VFX/Audio/SFX_Vefects_Explosion_Thermite_Once_Cue.SFX_Vefects_Explosion_Thermite_Once_Cue"))
        (:`NewEnumerator9`
          (`NiagaraComponent.SetAsset` _fx_3 "/Game/_ExternalAsset/Vefects/Explosions_VFX/VFX/Artillery/NS_ExplosionArtilleryLarge_Once.NS_ExplosionArtilleryLarge_Once" true)
          (`AudioComponent.SetSound` _sfx_2 "/Game/_ExternalAsset/Vefects/Explosions_VFX/Audio/SFX_Vefects_Explosion_Artillery_Cue.SFX_Vefects_Explosion_Artillery_Cue"))
        (:`NewEnumerator10`
          (`NiagaraComponent.SetAsset` _fx_3 "/Game/_ExternalAsset/Vefects/Explosions_VFX/VFX/Gasoline/NS_ExplosionGasolineLarge_Once.NS_ExplosionGasolineLarge_Once" true)
          (`AudioComponent.SetSound` _sfx_2 "/Game/_ExternalAsset/Vefects/Explosions_VFX/Audio/SFX_Vefects_Explosion_Gasoline_Cue.SFX_Vefects_Explosion_Gasoline_Cue"))))
    (:`NewEnumerator1`
      (`SceneComponent.K2_AddLocalOffset` _fx (`KismetMathLibrary.MakeVector` 0.0 0.0 (`self.Aerial Location Offset`)) false false)
      (switch `/Game/_ExternalAsset/Vefects/Explosions_VFX/Blueprints/BP_Enum_Explosion_Type` (`self.Select`)
        (:`NewEnumerator0`
          (`NiagaraComponent.SetAsset` _fx_2 "/Game/_ExternalAsset/Vefects/Explosions_VFX/VFX/Generic/BaseColors/NS_ExplosionGenericLarge_Aerial_Once.NS_ExplosionGenericLarge_Aerial_Once" true)
          (`AudioComponent.SetSound` _sfx "/Game/_ExternalAsset/Vefects/Explosions_VFX/Audio/SFX_Vefects_Explosion_Generic_Cue.SFX_Vefects_Explosion_Generic_Cue"))
        (:`NewEnumerator1`
          (`NiagaraComponent.SetAsset` _fx_2 "/Game/_ExternalAsset/Vefects/Explosions_VFX/VFX/Grenade/NS_ExplosionGrenade_Aerial_Once.NS_ExplosionGrenade_Aerial_Once" true)
          (`AudioComponent.SetSound` _sfx "/Game/_ExternalAsset/Vefects/Explosions_VFX/Audio/SFX_Vefects_Explosion_Grenade_Cue.SFX_Vefects_Explosion_Grenade_Cue"))
        (:`NewEnumerator2`
          (`NiagaraComponent.SetAsset` _fx_2 "/Game/_ExternalAsset/Vefects/Explosions_VFX/VFX/Molotov/NS_MolotovExplosion_Aerial_Once.NS_MolotovExplosion_Aerial_Once" true)
          (`AudioComponent.SetSound` _sfx "/Game/_ExternalAsset/Vefects/Explosions_VFX/Audio/SFX_Vefects_Explosion_Incendiary_Cue.SFX_Vefects_Explosion_Incendiary_Cue"))
        (:`NewEnumerator3`
          (`NiagaraComponent.SetAsset` _fx_2 "/Game/_ExternalAsset/Vefects/Explosions_VFX/VFX/Generic/Toxic/NS_ExplosionGenericLarge_Aerial_Toxic_Once.NS_ExplosionGenericLarge_Aerial_Toxic_Once" true)
          (`AudioComponent.SetSound` _sfx "/Game/_ExternalAsset/Vefects/Explosions_VFX/Audio/SFX_Vefects_Explosion_Hellfire_Cue.SFX_Vefects_Explosion_Hellfire_Cue"))
        (:`NewEnumerator4`
          (`NiagaraComponent.SetAsset` _fx_2 "/Game/_ExternalAsset/Vefects/Explosions_VFX/VFX/Generic/BlackBody/NS_ExplosionGenericLarge_Aerial_Blackbody_Once.NS_ExplosionGenericLarge_Aerial_Blackbody_Once" true)
          (`AudioComponent.SetSound` _sfx "/Game/_ExternalAsset/Vefects/Explosions_VFX/Audio/SFX_Vefects_Explosion_Black_Cue.SFX_Vefects_Explosion_Black_Cue"))
        (:`NewEnumerator5`
          (`NiagaraComponent.SetAsset` _fx_2 "/Game/_ExternalAsset/Vefects/Explosions_VFX/VFX/Sci-Fi/NS_ElectricExplosion_Aerial_Once.NS_ElectricExplosion_Aerial_Once" true)
          (`AudioComponent.SetSound` _sfx "/Game/_ExternalAsset/Vefects/Explosions_VFX/Audio/SFX_Vefects_Explosion_Electric_Cue.SFX_Vefects_Explosion_Electric_Cue"))
        (:`NewEnumerator6`
          (`NiagaraComponent.SetAsset` _fx_2 "/Game/_ExternalAsset/Vefects/Explosions_VFX/VFX/GasGrenade/NS_GasGrenade_Medium_Aerial_Once.NS_GasGrenade_Medium_Aerial_Once" true)
          (`AudioComponent.SetSound` _sfx "/Game/_ExternalAsset/Vefects/Explosions_VFX/Audio/SFX_Vefects_Explosion_Gas_Cue.SFX_Vefects_Explosion_Gas_Cue"))
        (:`NewEnumerator7`
          (`NiagaraComponent.SetAsset` _fx_2 "/Game/_ExternalAsset/Vefects/Explosions_VFX/VFX/Water/NS_WaterExplosion_Once.NS_WaterExplosion_Once" true)
          (`AudioComponent.SetSound` _sfx "/Game/_ExternalAsset/Vefects/Explosions_VFX/Audio/SFX_Vefects_Explosion_Water_Cue.SFX_Vefects_Explosion_Water_Cue"))
        (:`NewEnumerator8`
          (`NiagaraComponent.SetAsset` _fx_2 "/Game/_ExternalAsset/Vefects/Explosions_VFX/VFX/Thermite/NS_ThermiteGrenade_Once.NS_ThermiteGrenade_Once" true)
          (`AudioComponent.SetSound` _sfx "/Game/_ExternalAsset/Vefects/Explosions_VFX/Audio/SFX_Vefects_Explosion_Thermite_Once_Cue.SFX_Vefects_Explosion_Thermite_Once_Cue"))
        (:`NewEnumerator9`
          (`NiagaraComponent.SetAsset` _fx_2 "/Game/_ExternalAsset/Vefects/Explosions_VFX/VFX/Artillery/NS_ExplosionArtilleryLarge_Once.NS_ExplosionArtilleryLarge_Once" true)
          (`AudioComponent.SetSound` _sfx "/Game/_ExternalAsset/Vefects/Explosions_VFX/Audio/SFX_Vefects_Explosion_Artillery_Cue.SFX_Vefects_Explosion_Artillery_Cue"))
        (:`NewEnumerator10`
          (`NiagaraComponent.SetAsset` _fx_2 "/Game/_ExternalAsset/Vefects/Explosions_VFX/VFX/Gasoline/NS_ExplosionGasolineLarge_Aerial_Once.NS_ExplosionGasolineLarge_Aerial_Once" true)
          (`AudioComponent.SetSound` _sfx "/Game/_ExternalAsset/Vefects/Explosions_VFX/Audio/SFX_Vefects_Explosion_Gasoline_Cue.SFX_Vefects_Explosion_Gasoline_Cue"))))))
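; BP_TargetShip is a target ship from the Space VFX pack that shows an energy shield impact effect when hit.
; ShieldHit spawns an attached Niagara shield effect scaled to the EnergyShield, stores the hit's offset from the root and plays an impact sound.
; Tick re-feeds that offset as a world HitPosition so the impact follows the ship.
; A looping movement timeline exists but is unconnected, and StartMoving is empty.
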(event `self.ReceiveBeginPlay`
  (`self.StartMoving`))

(event `StartMoving`)

(event `self.ReceiveTick`
  (params (DeltaSeconds :type "Float (single-precision)"))
  (if (`KismetSystemLibrary.IsValid` (`self.ShieldHitEffect`))
    (`NiagaraComponent.SetVariableVec3` (`self.ShieldHitEffect`) "HitPosition" (+ (`SceneComponent.K2_GetComponentLocation` (`self.DefaultSceneRoot`)) (`self.ShieldHitRelativeOffset`)))))

(event `ShieldHit`
  (bind _returnvalue (`NiagaraFunctionLibrary.SpawnSystemAttached` "/Game/_ExternalAsset/Vefects/Space_VFX/VFX/Shields/NS_EnergyShield.NS_EnergyShield" (`self.DefaultSceneRoot`) "None" (0.0 0.0 0.0) (struct) "KeepRelativeOffset"))
  (set `self.ShieldHitEffect` _returnvalue)
  (set `self.ShieldHitRelativeOffset` (- (`self.ShieldHitPosition`) (`SceneComponent.K2_GetComponentLocation` (`self.DefaultSceneRoot`))))
  (`NiagaraComponent.SetVariableVec3` (`self.ShieldHitEffect`) "ShieldScale" (`SceneComponent.RelativeScale3D` (`self.EnergyShield`)))
  (`GameplayStatics.SpawnSoundAtLocation` "/Game/_ExternalAsset/Vefects/Space_VFX/Audio/SFX_Vefects_Space_Shield_Impact_Cue.SFX_Vefects_Space_Shield_Impact_Cue" (`self.K2_GetActorLocation`) (struct) 0.5 1.0 0.0 null null))

(fn `UserConstructionScript`)
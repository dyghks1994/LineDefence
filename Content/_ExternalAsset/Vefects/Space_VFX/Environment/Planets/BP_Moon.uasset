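; BP_Moon is a moon actor from the Vefects Space VFX environment planets, with a StaticMesh and a Pivot component.
; Three timelines are wired to turn Pivot a full 360 degrees by lerping pitch, roll or yaw, with the pitch one also spinning StaticMesh.
; None of these timelines is triggered, and BeginPlay and the construction script are empty, so this graph leaves the moon static.
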(event `self.ReceiveBeginPlay`)

(fn `UserConstructionScript`)
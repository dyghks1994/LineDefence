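; Slime projectile VFX actor from the Vefects pack that pairs a static mesh with three Niagara effects for the surface, drips and moving drips.
; The construction script switches on Type to set the mesh material and all three Niagara assets to either standard or transparent variants, with standard as the default.
; The event graph holds only disabled placeholder events, so this Blueprint adds no movement or hit logic in its graphs.
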(fn `UserConstructionScript`
  (bind _staticmesh (`self.StaticMesh`))
  (bind _ns_slime_surface_01 (`self.NS_Slime_Surface_01`))
  (bind _ns_slime_surface_drips_01 (`self.NS_Slime_Surface_Drips_01`))
  (bind _ns_slime_surface_drips_01_move (`self.NS_Slime_Surface_Drips_01_Move`))
  (switch `int` (`self.Type`)
    (:`Default`
      (`PrimitiveComponent.SetMaterial` _staticmesh 0 "/Game/_ExternalAsset/Vefects/Slime_VFX/Slime/Materials/MI_VFX_Slime_Projectile_01.MI_VFX_Slime_Projectile_01" :!label _label)
      (`NiagaraComponent.SetAsset` _ns_slime_surface_01 "/Game/_ExternalAsset/Vefects/Slime_VFX/Slime/Particles/NS_Slime_Surface_01.NS_Slime_Surface_01" true)
      (`NiagaraComponent.SetAsset` _ns_slime_surface_drips_01 "/Game/_ExternalAsset/Vefects/Slime_VFX/Slime/Particles/NS_Slime_Surface_Drips_01.NS_Slime_Surface_Drips_01" true)
      (`NiagaraComponent.SetAsset` _ns_slime_surface_drips_01_move "/Game/_ExternalAsset/Vefects/Slime_VFX/Slime/Particles/NS_Slime_Surface_Drips_01_Move.NS_Slime_Surface_Drips_01_Move" true))
    (:`0`
      (goto _label))
    (:`1`
      (`PrimitiveComponent.SetMaterial` _staticmesh 0 "/Game/_ExternalAsset/Vefects/Slime_VFX/Slime/Materials/MI_VFX_Slime_Projectile_Transparent_01.MI_VFX_Slime_Projectile_Transparent_01")
      (`NiagaraComponent.SetAsset` _ns_slime_surface_01 "/Game/_ExternalAsset/Vefects/Slime_VFX/Slime/Particles/NS_Slime_Surface_01_Transparent.NS_Slime_Surface_01_Transparent" true)
      (`NiagaraComponent.SetAsset` _ns_slime_surface_drips_01 "/Game/_ExternalAsset/Vefects/Slime_VFX/Slime/Particles/NS_Slime_Surface_Drips_01_Transparent.NS_Slime_Surface_Drips_01_Transparent" true)
      (`NiagaraComponent.SetAsset` _ns_slime_surface_drips_01_move "/Game/_ExternalAsset/Vefects/Slime_VFX/Slime/Particles/NS_Slime_Surface_Drips_01_Transparent_Move.NS_Slime_Surface_Drips_01_Transparent_Move" true))))
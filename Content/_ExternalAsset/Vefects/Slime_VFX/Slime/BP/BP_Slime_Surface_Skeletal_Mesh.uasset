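; Slime surface VFX actor that spawns a Niagara slime effect on a configurable skeletal mesh.
; The construction script picks the opaque or transparent Niagara system from the Transparent setting and assigns the custom skeletal mesh to the SkeletalMesh component.
; It sets a white material on the mesh's first slot, then binds that component to the Niagara system's User.SkeletalMesh parameter.
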(fn `UserConstructionScript`
  (bind _skeletalmesh (`self.SkeletalMesh`))
  (bind _niagara (`self.Niagara`))
  (switch `int` (`self.Transparent`)
    (:`Default`
      (`NiagaraComponent.SetAsset` _niagara "/Game/_ExternalAsset/Vefects/Slime_VFX/Slime/Particles/NS_Slime_Surface_Spawn_Skeletal_Mesh_01.NS_Slime_Surface_Spawn_Skeletal_Mesh_01" true :!label _label))
    (:`0`
      (goto _label))
    (:`1`
      (`NiagaraComponent.SetAsset` _niagara "/Game/_ExternalAsset/Vefects/Slime_VFX/Slime/Particles/NS_Slime_Surface_Spawn_Skeletal_Mesh_01_Transparent.NS_Slime_Surface_Spawn_Skeletal_Mesh_01_Transparent" true)))
  (`SkinnedMeshComponent.SetSkinnedAssetAndUpdate` _skeletalmesh (`self.CustomSkeletalMesh`) true)
  (`|ExecutionSequence`
    (:`then_0`
      (`PrimitiveComponent.SetMaterial` _skeletalmesh 0 "/Game/_ExternalAsset/Vefects/Slime_VFX/Demo/Resources/Materials/M_White.M_White"))
    (:`then_1`
      (`NiagaraFunctionLibrary.OverrideSystemUserVariableSkeletalMeshComponent` (`self.Niagara`) "User.SkeletalMesh" (`self.SkeletalMesh`)))))
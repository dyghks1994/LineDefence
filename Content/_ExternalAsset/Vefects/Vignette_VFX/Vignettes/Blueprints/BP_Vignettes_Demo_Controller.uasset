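; Demo controller Blueprint for previewing the Vefects screen vignette effects by keyboard.
; Add and Subtract keys step a selected vignette ID, clamped to the range of available effects, then refresh the on-screen name through a switch from ID to label.
; F asks the VignettesManager to play the selected vignette, and G calls the same function with its turn-off flag set.
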(event `Key|Add`
  (params (Key :type "Key Structure"))
  (:`Pressed`
    (bind _result (`/Engine/EditorBlueprintResources/StandardMacros.IncrementInt` (`self.Currently Selected Vignette ID`))
      (:`  `
        (set `self.Currently Selected Vignette ID` (`KismetMathLibrary.Clamp` _result 1 20))
        (`self.Update Selected Vignette Text`)))))

(event `Key|F`
  (params (Key :type "Key Structure"))
  (:`Pressed`
    (`/Game/_ExternalAsset/Vefects/Vignette_VFX/Vignettes/Blueprints/BP_Vignettes_Manager.Call Vignette` (`self.Vignettes_Manager`) (`self.Currently Selected Vignette ID`) 1000000000.0 false false)))

(event `Key|Subtract`
  (params (Key :type "Key Structure"))
  (:`Pressed`
    (bind _result (`/Engine/EditorBlueprintResources/StandardMacros.DecrementInt` (`self.Currently Selected Vignette ID`))
      (:`  `
        (set `self.Currently Selected Vignette ID` (`KismetMathLibrary.Clamp` _result 1 20))
        (`self.Update Selected Vignette Text`)))))

(event `Key|G`
  (params (Key :type "Key Structure"))
  (:`Pressed`
    (`/Game/_ExternalAsset/Vefects/Vignette_VFX/Vignettes/Blueprints/BP_Vignettes_Manager.Call Vignette` (`self.Vignettes_Manager`) (`self.Currently Selected Vignette ID`) 1000000000.0 false true)))

(event `Update Selected Vignette Text`
  (switch `int` (`self.Currently Selected Vignette ID`)
    (:`Default`
      (set `self.Selected Vignette Name` "Undefined" :!label _label))
    (:`0`
      (goto _label))
    (:`1`
      (set `self.Selected Vignette Name` "Water"))
    (:`2`
      (set `self.Selected Vignette Name` "Burning"))
    (:`3`
      (set `self.Selected Vignette Name` "Hurt"))
    (:`4`
      (set `self.Selected Vignette Name` "Poisoned"))
    (:`5`
      (set `self.Selected Vignette Name` "Sci-fi Shield"))
    (:`6`
      (set `self.Selected Vignette Name` "Speed"))
    (:`7`
      (set `self.Selected Vignette Name` "Speed (Anime)"))
    (:`8`
      (set `self.Selected Vignette Name` "Frozen"))
    (:`9`
      (set `self.Selected Vignette Name` "Drunk"))
    (:`10`
      (set `self.Selected Vignette Name` "Charmed"))
    (:`11`
      (set `self.Selected Vignette Name` "Glitch"))
    (:`12`
      (set `self.Selected Vignette Name` "Glitch (Strong)"))
    (:`13`
      (set `self.Selected Vignette Name` "Glitch (Borders Only)"))
    (:`14`
      (set `self.Selected Vignette Name` "Healed"))
    (:`15`
      (set `self.Selected Vignette Name` "Fear"))
    (:`16`
      (set `self.Selected Vignette Name` "Goo"))
    (:`17`
      (set `self.Selected Vignette Name` "Puke"))
    (:`18`
      (set `self.Selected Vignette Name` "Poo"))
    (:`19`
      (set `self.Selected Vignette Name` "Muddy"))
    (:`20`
      (set `self.Selected Vignette Name` "Bloody")))
  (`TextRenderComponent.K2_SetText` (`self.SelectedVignette`) (`self.Selected Vignette Name`)))

(fn `UserConstructionScript`)
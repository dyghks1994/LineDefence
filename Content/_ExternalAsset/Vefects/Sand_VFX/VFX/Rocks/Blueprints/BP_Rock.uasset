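; Rock actor from the Vefects Sand VFX pack that plays an eruption cast sound on spawn and breaks apart on hit.
; On hit, it spawns a Niagara impact at the mesh location, passing the mesh velocity as InitialVelocity so the effect can inherit its motion.
; It plays one of three random hit sounds, destroys the mesh immediately, then destroys the actor after a short delay.
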(event `self.ReceiveBeginPlay`
  (`GameplayStatics.SpawnSoundAtLocation` "/Game/_ExternalAsset/Vefects/Sand_VFX/Audio/SFX_Vefects_Sand_Rock_Eruption_Cast_Cue.SFX_Vefects_Sand_Rock_Eruption_Cast_Cue" (`self.K2_GetActorLocation`) (struct) 1.0 1.0 0.0 "/Game/_ExternalAsset/Vefects/Sand_VFX/Audio/SFX_Attenuation.SFX_Attenuation" null))

(event `self.ReceiveHit`
  (params (MyComp :type "PrimitiveComponent Object Reference") (Other :type "Actor Object Reference") (OtherComp :type "PrimitiveComponent Object Reference") (bSelfMoved :type Boolean) (HitLocation :type "Vector Structure") (HitNormal :type "Vector Structure") (NormalImpulse :type "Vector Structure") (Hit :type "HitResult Structure (by ref)"))
  (bind _returnvalue (`NiagaraFunctionLibrary.SpawnSystemAtLocation` "/Game/_ExternalAsset/Vefects/Sand_VFX/VFX/Rocks/NS_Rock_Impact.NS_Rock_Impact" (`SceneComponent.K2_GetComponentLocation` (`self.StaticMesh`))))
  (`FXSystemComponent.SetVectorParameter` _returnvalue "InitialVelocity" (`SceneComponent.GetComponentVelocity` (`self.StaticMesh`)))
  (`|ExecutionSequence`
    (:`then_0`
      (switch `int` (`KismetMathLibrary.RandomIntegerInRange` 0 2)
        (:`Default`
          (`GameplayStatics.SpawnSoundAtLocation` "/Game/_ExternalAsset/Vefects/Sand_VFX/Audio/SFX_Vefects_Sand_Rock_Hit_01_Cue.SFX_Vefects_Sand_Rock_Hit_01_Cue" HitLocation (struct) 1.0 1.0 0.0 "/Game/_ExternalAsset/Vefects/Sand_VFX/Audio/SFX_Attenuation.SFX_Attenuation" null :!label _label))
        (:`0`
          (goto _label))
        (:`1`
          (`GameplayStatics.SpawnSoundAtLocation` "/Game/_ExternalAsset/Vefects/Sand_VFX/Audio/SFX_Vefects_Sand_Rock_Hit_02_Cue.SFX_Vefects_Sand_Rock_Hit_02_Cue" HitLocation (struct) 1.0 1.0 0.0 "/Game/_ExternalAsset/Vefects/Sand_VFX/Audio/SFX_Attenuation.SFX_Attenuation" null))
        (:`2`
          (`GameplayStatics.SpawnSoundAtLocation` "/Game/_ExternalAsset/Vefects/Sand_VFX/Audio/SFX_Vefects_Sand_Rock_Eruption_Hit_Cue.SFX_Vefects_Sand_Rock_Eruption_Hit_Cue" HitLocation (struct) 1.0 1.0 0.0 "/Game/_ExternalAsset/Vefects/Sand_VFX/Audio/SFX_Attenuation.SFX_Attenuation" null))))
    (:`then_1`
      (`ActorComponent.K2_DestroyComponent` (`self.StaticMesh`))
      (`KismetSystemLibrary.Delay` 2.0)
      (`self.K2_DestroyActor`))))

(fn `UserConstructionScript`)
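; Scene capture actor that follows player character 0 in XY to maintain render targets for the dynamic sand surface effect.
; BeginPlay clears both sand targets, creates the draw material, computes world-space pixel size and publishes capture size to MPC_DynamicSand.
; Tick moves the actor in pixel-snapped steps, publishes its location, then draws into the persistent target with the normalized movement offset to compensate for scrolling.
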(event `self.ReceiveBeginPlay`
  (`KismetMaterialLibrary.SetScalarParameterValue` "/Game/_ExternalAsset/Vefects/Sand_VFX/VFX/DynamicSandSurface/Materials/MPC_DynamicSand.MPC_DynamicSand" "CaptureSize" (`SceneCaptureComponent2D.OrthoWidth` (`self.SceneCaptureComponent2D`)))
  (bind _returnvalue (`KismetMaterialLibrary.CreateDynamicMaterialInstance` "/Game/_ExternalAsset/Vefects/Sand_VFX/VFX/DynamicSandSurface/Materials/M_VFX_Draw_To_Persistent_RT.M_VFX_Draw_To_Persistent_RT"))
  (set `self.Draw_Material` _returnvalue)
  (`KismetRenderingLibrary.ClearRenderTarget2D` "/Game/_ExternalAsset/Vefects/Sand_VFX/VFX/DynamicSandSurface/Textures/RT_Dynamic_Sand.RT_Dynamic_Sand")
  (`KismetRenderingLibrary.ClearRenderTarget2D` "/Game/_ExternalAsset/Vefects/Sand_VFX/VFX/DynamicSandSurface/Textures/RT_Dynamic_Sand_Persistent.RT_Dynamic_Sand_Persistent")
  (set `self.PixelSizeWS` (* (`SceneCaptureComponent2D.OrthoWidth` (`self.SceneCaptureComponent2D`)) (/ 1.0 (`self.RenderTargetResolution`)))))

(event `self.ReceiveTick`
  (params (DeltaSeconds :type "Float (single-precision)"))
  (bind (_returnvalue_x _returnvalue_y) (`KismetMathLibrary.BreakVector` (`self.K2_GetActorLocation`)))
  (bind _pixelsizews (`self.PixelSizeWS`))
  (bind _pixelsizews_2 (`self.PixelSizeWS`))
  (bind (_returnvalue_x_2 _returnvalue_y_2) (`KismetMathLibrary.BreakVector` (`self.K2_GetActorLocation` (`GameplayStatics.GetPlayerCharacter` 0))))
  (bind (_returnvalue_x_3 _returnvalue_y_3) (`KismetMathLibrary.BreakVector2D` (/ (`self.CaptureOffset`) (`SceneCaptureComponent2D.OrthoWidth` (`self.SceneCaptureComponent2D`)))))
  (bind _output_get (set `self.CaptureOffset` (- (`KismetMathLibrary.MakeVector2D` (* (`KismetMathLibrary.FFloor` (+ (/ _returnvalue_x_2 _pixelsizews_2) 0.5)) _pixelsizews_2) (* (`KismetMathLibrary.FFloor` (+ (/ _returnvalue_y_2 _pixelsizews) 0.5)) _pixelsizews)) (`KismetMathLibrary.MakeVector2D` _returnvalue_x _returnvalue_y))))
  (`self.K2_AddActorWorldOffset` (`KismetMathLibrary.MakeVector` (`KismetMathLibrary.BreakVector2D` _output_get) (`.Y` (`KismetMathLibrary.BreakVector2D` _output_get))))
  (`KismetMaterialLibrary.SetVectorParameterValue` "/Game/_ExternalAsset/Vefects/Sand_VFX/VFX/DynamicSandSurface/Materials/MPC_DynamicSand.MPC_DynamicSand" "CaptureLocation" (`KismetMathLibrary.Conv_VectorToLinearColor` (`self.K2_GetActorLocation`)))
  (`MaterialInstanceDynamic.SetVectorParameterValue` (`self.Draw_Material`) "Offset" (make `LinearColor` _returnvalue_x_3 _returnvalue_y_3 0.0 1.0))
  (`KismetRenderingLibrary.DrawMaterialToRenderTarget` "/Game/_ExternalAsset/Vefects/Sand_VFX/VFX/DynamicSandSurface/Textures/RT_Dynamic_Sand_Persistent.RT_Dynamic_Sand_Persistent" (`self.Draw_Material`)))

(fn `UserConstructionScript`)
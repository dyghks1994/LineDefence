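; Demo pressure washer actor that shoots a water stream mesh with a Niagara impact effect where it hits.
; Each tick while on, a short forward line trace scales the stream mesh and its material length to the hit distance.
; The trace also places the impact effect and feeds it the hit normal, width and spawn flag.
; It either sweeps automatically on a looping timeline or, in first-person mode, follows the camera and sprays while left mouse is held.
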(event `self.ReceiveBeginPlay`
  (bind _returnvalue (`PrimitiveComponent.CreateDynamicMaterialInstance` (`self.WaterStream`) 0 null "None"))
  (set `self.WaterStreamDynamicMaterialInstance` _returnvalue)
  (if (not (`self.First Person Mode`))
    (set `self.isTurnedOn?` true)
    ;[1 1 1] Moves the hose around, for demo purposes
    (bind (_direction _curve _curveshorter) (`Timeline|Position` :!via `PlayFromStart` :!label _label)
      (:`Update`
        (`self.K2_SetActorRotation` (`KismetMathLibrary.MakeRotator` 0.0 (* _curveshorter 20.0) 90.0))
        (`self.K2_SetActorLocation` (+ (`self.InitialLocation`) (`KismetMathLibrary.MakeVector` (* _curve 200.0)))))
      (:`Finished`
        (goto _label :!via `PlayFromStart`)))))

(event `self.ReceiveTick`
  (params (DeltaSeconds :type "Float (single-precision)"))
  (bind _waterstream (`self.WaterStream`))
  (bind _streamscalexpercentage (`self.StreamScaleXPercentage`))
  (bind _returnvalue (`SceneComponent.K2_GetComponentLocation` _waterstream))
  (if (`self.First Person Mode`)
    ;[1 1 1] First person controls
    (`self.K2_SetActorLocation` (+ (+ (`PlayerCameraManager.GetCameraLocation` (`GameplayStatics.GetPlayerCameraManager` 0)) (* (`KismetMathLibrary.GetUpVector` (`PlayerCameraManager.GetCameraRotation` (`GameplayStatics.GetPlayerCameraManager` 0))) -15.0)) (* (`KismetMathLibrary.GetRightVector` (`PlayerCameraManager.GetCameraRotation` (`GameplayStatics.GetPlayerCameraManager` 0))) 15.0)))
    (`self.K2_SetActorRotation` (`PlayerCameraManager.GetCameraRotation` (`GameplayStatics.GetPlayerCameraManager` 0))))
  (if (`self.isTurnedOn?`)
    (bind (_outhit _returnvalue_2) (`KismetSystemLibrary.LineTraceSingle` _returnvalue (+ _returnvalue (* (`SceneComponent.GetForwardVector` _waterstream) 300.0)) "TraceTypeQuery1"))
    (set `self.ShouldParticlesSpawn?` _returnvalue_2)
    (if _returnvalue_2
      (bind (_bblockinghit _binitialoverlap _time _distance _location _impactpoint _normal _impactnormal) (`GameplayStatics.BreakHitResult` _outhit))
      (set `self.HitDistance` _distance)
      (set `self.HitLocation` _location)
      (set `self.Impact Normal` _impactnormal)
      (set `self.StreamScaleXPercentage` (`KismetMathLibrary.FClamp` (/ (`self.HitDistance`) 300.0)))
      (`SceneComponent.K2_SetWorldLocation` (`self.NS_PressureWasherImpactCenter`) (`self.HitLocation`) false false)
      (`FXSystemComponent.SetVectorParameter` (`self.NS_PressureWasherImpactCenter`) "HitNormal" (`self.Impact Normal`))
      (else
        (set `self.StreamScaleXPercentage` 1.0)
        (`FXSystemComponent.SetBoolParameter` (`self.NS_PressureWasherImpactCenter`) "ShouldSpawn" false)))
    (else
      (set `self.StreamScaleXPercentage` 0.0)
      (set `self.ShouldParticlesSpawn?` false)))
  (`SceneComponent.SetRelativeScale3D` (`self.WaterStream`) (`KismetMathLibrary.MakeVector` _streamscalexpercentage _streamscalexpercentage 1.0))
  (`MaterialInstanceDynamic.SetScalarParameterValue` (`self.WaterStreamDynamicMaterialInstance`) "StreamLengthPercentage" (`self.StreamScaleXPercentage`))
  (`FXSystemComponent.SetBoolParameter` (`self.NS_PressureWasherImpactCenter`) "ShouldSpawn" (`self.ShouldParticlesSpawn?`))
  (`FXSystemComponent.SetFloatParameter` (`self.NS_PressureWasherImpactCenter`) "Width" (* (`self.StreamScaleXPercentage`) 100.0)))

(event `Key|LeftMouseButton`
  (params (Key :type "Key Structure"))
  ;[1 1 1] First person controls
  (:`Pressed`
    (if (`self.First Person Mode`)
      (set `self.isTurnedOn?` true)))
  (:`Released`
    (if (`self.First Person Mode`)
      (set `self.isTurnedOn?` false))))

(fn `UserConstructionScript`
  (set `self.InitialLocation` (`self.K2_GetActorLocation`)))
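; BP_GardenHose is a demo actor for a Niagara garden hose water stream from the Vefects Water VFX pack.
; The construction script passes StreamStrength to the stream's HoseStrength parameter and caches the actor's starting location.
; On BeginPlay, a self-restarting Position timeline pitches the hose and slides it along X from that location to show the stream in motion.
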(event `self.ReceiveBeginPlay`
  ;[1 1 1] Moves the hose around, for demo purposes
  (bind (_direction _curve _curveshorter) (`Timeline|Position` :!via `PlayFromStart` :!label _label)
    (:`Update`
      (`self.K2_SetActorRotation` (`KismetMathLibrary.MakeRotator` 0.0 (* _curve -30.0) 90.0))
      (`self.K2_SetActorLocation` (+ (`self.InitialLocation`) (`KismetMathLibrary.MakeVector` (* _curveshorter 50.0)))))
    (:`Finished`
      (goto _label :!via `PlayFromStart`))))

(fn `UserConstructionScript`
  (`FXSystemComponent.SetFloatParameter` (`self.NS_GardenHoseStream`) "HoseStrength" (`self.Stream Strength`))
  (set `self.InitialLocation` (`self.K2_GetActorLocation`)))
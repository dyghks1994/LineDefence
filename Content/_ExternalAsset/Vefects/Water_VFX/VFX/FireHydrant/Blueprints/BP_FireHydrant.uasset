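; Fire hydrant VFX actor from the Vefects Water pack, toggled on and off with the H key along with start, loop and end sounds.
; Tick ramps an on/off value, rising faster than it falls, and remaps it through a curve.
; That value drives the stream mesh's scale and StreamStrength material parameter, plus the Niagara splashes' spawn rate and stream top position along the actor's up vector.
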(event `self.ReceiveBeginPlay`
  (bind _returnvalue (`PrimitiveComponent.CreateDynamicMaterialInstance` (`self.SM_FireHydrantMainStream`) 0 null "None"))
  (set `self.FireHydrantMainStreamDynamicMaterialInstance` _returnvalue))

(event `self.ReceiveTick`
  (params (DeltaSeconds :type "Float (single-precision)"))
  (bind _turnedonindicatorremapped (`self.TurnedOnIndicatorRemapped`))
  (set `self.Delta Seconds` DeltaSeconds)
  (if (`self.isTurnedOn?`)
    (bind _output_get (set `self.TurnedOnIndicatorLinear` (`KismetMathLibrary.FClamp` (+ (`self.TurnedOnIndicatorLinear`) (* (`self.Delta Seconds`) 5.0)))))
    (set `self.TurnedOnIndicatorRemapped` (`CurveFloat.GetFloatValue` (`self.C_Cubic`) _output_get))
    (else
      (bind _output_get_2 (set `self.TurnedOnIndicatorLinear` (`KismetMathLibrary.FClamp` (- (`self.TurnedOnIndicatorLinear`) (* (`self.Delta Seconds`) 1.0)))))
      (set `self.TurnedOnIndicatorRemapped` (`CurveFloat.GetFloatValue` (`self.C_Cubic`) _output_get_2))))
  (`SceneComponent.SetRelativeScale3D` (`self.SM_FireHydrantMainStream`) (`KismetMathLibrary.MakeVector` _turnedonindicatorremapped _turnedonindicatorremapped _turnedonindicatorremapped))
  (`FXSystemComponent.SetVectorParameter` (`self.NS_FireHydrantSplashes`) "StreamBottom" (`self.K2_GetActorLocation`))
  (`FXSystemComponent.SetVectorParameter` (`self.NS_FireHydrantSplashes`) "StreamTop" (+ (`self.K2_GetActorLocation`) (* (`self.GetActorUpVector`) (* (`self.TurnedOnIndicatorRemapped`) 300.0))))
  (`FXSystemComponent.SetFloatParameter` (`self.NS_FireHydrantSplashes`) "SpawnRateMult" (`self.TurnedOnIndicatorRemapped`))
  (`MeshComponent.SetScalarParameterValueOnMaterials` (`self.SM_FireHydrantMainStream`) "StreamStrength" (`self.TurnedOnIndicatorRemapped`)))

(event `Key|H`
  (params (Key :type "Key Structure"))
  (bind _sfx_vefects_water_fire_hydrant_loop_cue (`self.SFX_Vefects_Water_Fire_Hydrant_Loop_Cue`))
  (:`Pressed`
    (if (`self.isTurnedOn?`)
      (set `self.isTurnedOn?` false)
      (`AudioComponent.Play` (`self.SFX_Vefects_Water_Fire_Hydrant_End_Cue`) 0.0)
      (`AudioComponent.FadeOut` _sfx_vefects_water_fire_hydrant_loop_cue 0.5 0.0 "Linear")
      (else
        (set `self.isTurnedOn?` true)
        (`AudioComponent.Play` (`self.SFX_Vefects_Water_Fire_Hydrant_Cast_Cue`) 0.0)
        (`KismetSystemLibrary.Delay` 1.0)
        (`AudioComponent.Play` _sfx_vefects_water_fire_hydrant_loop_cue 0.0)))))

(fn `UserConstructionScript`
  (`FXSystemComponent.SetVectorParameter` (`self.NS_FireHydrantSplashes`) "StreamBottom" (`self.K2_GetActorLocation`))
  (`FXSystemComponent.SetVectorParameter` (`self.NS_FireHydrantSplashes`) "StreamTop" (+ (`self.K2_GetActorLocation`) (* (`self.GetActorUpVector`) (* (`self.TurnedOnIndicatorLinear`) 300.0)))))
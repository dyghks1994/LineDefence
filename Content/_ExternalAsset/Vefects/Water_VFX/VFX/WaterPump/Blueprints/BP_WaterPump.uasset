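; Water pump VFX actor with a falling stream, splashes and optional puddle decal, toggled on and off with the P key.
; Construction traces down to place the Niagara effect and puddle on the surface below and sets stream height from the hit distance.
; Toggling switches splashes and plays start, loop and end sounds.
; Tick ramps a stream-width value, faster opening than closing, that also drives puddle wave intensity.
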(event `self.ReceiveBeginPlay`)

(event `Key|P`
  (params (Key :type "Key Structure"))
  (:`Pressed`
    (if (`self.isTurnedOn?`)
      (`self.TurnOff`)
      (else
        (`self.TurnOn`)))))

(event `TurnOn`
  (if (not (`self.isTurnedOn?`))
    (`FXSystemComponent.SetBoolParameter` (`self.NS_WaterPump`) "SpawnSplashes" true)
    (set `self.isTurnedOn?` true)
    (`AudioComponent.Play` (`self.SFX_Vefects_Water_Pump_Cast_Cue`) 0.0)
    (`KismetSystemLibrary.Delay` 1.0)
    (`AudioComponent.Play` (`self.SFX_Vefects_Water_Pump_Loop_Cue`) 0.0)))

(event `TurnOff`
  (if (`self.isTurnedOn?`)
    (`FXSystemComponent.SetBoolParameter` (`self.NS_WaterPump`) "SpawnSplashes" false)
    (set `self.isTurnedOn?` false)
    (`AudioComponent.Play` (`self.SFX_Vefects_Water_Pump_End_Cue`) 0.0)
    (`AudioComponent.FadeOut` (`self.SFX_Vefects_Water_Pump_Loop_Cue`) 0.5 0.0 "Linear")))

(event `self.ReceiveTick`
  (params (DeltaSeconds :type "Float (single-precision)"))
  (set `self.Delta Seconds` DeltaSeconds)
  (if (`self.isTurnedOn?`)
    (set `self.WaterStreamWidthPercentage` (`KismetMathLibrary.FClamp` (+ (`self.WaterStreamWidthPercentage`) (* (`self.Delta Seconds`) 7.5))))
    (else
      (set `self.WaterStreamWidthPercentage` (`KismetMathLibrary.FClamp` (- (`self.WaterStreamWidthPercentage`) (* (`self.Delta Seconds`) 3.0))))))
  (`FXSystemComponent.SetFloatParameter` (`self.NS_WaterPump`) "WaterStreamWidthPercentage" (`self.WaterStreamWidthPercentage`))
  (`MaterialInstanceDynamic.SetScalarParameterValue` (`self.PuddleDynamicMaterialInstance`) "WavesIntensity" (`self.WaterStreamWidthPercentage`)))

(fn `UserConstructionScript`
  (bind _returnvalue (`self.K2_GetActorLocation`))
  (bind _returnvalue_2 (`DecalComponent.CreateDynamicMaterialInstance` (`self.PuddleDecal`)))
  (set `self.PuddleDynamicMaterialInstance` _returnvalue_2)
  (if (not (`self.StartTurnedOn?`))
    (`MaterialInstanceDynamic.SetScalarParameterValue` (`self.PuddleDynamicMaterialInstance`) "WavesIntensity" 0.0)
    (set `self.WaterStreamWidthPercentage` 0.0)
    (`FXSystemComponent.SetBoolParameter` (`self.NS_WaterPump`) "SpawnSplashes" false)
    (set `self.isTurnedOn?` false))
  (bind (_outhit _returnvalue_3) (`KismetSystemLibrary.LineTraceSingle` _returnvalue (+ _returnvalue (0.0 0.0 -500.0)) "TraceTypeQuery1"))
  (if _returnvalue_3
    (bind (_bblockinghit _binitialoverlap _time _distance _location) (`GameplayStatics.BreakHitResult` _outhit))
    (`SceneComponent.K2_SetWorldLocation` (`self.NS_WaterPump`) _location false false)
    (`FXSystemComponent.SetFloatParameter` (`self.NS_WaterPump`) "Height" _distance)
    (`FXSystemComponent.SetFloatParameter` (`self.NS_WaterPump`) "Water Stream Width" (`self.WaterStreamMaxWidth`))
    (`FXSystemComponent.SetFloatParameter` (`self.NS_WaterPump`) "Splash Size" (`self.SplashSize`))
    (`FXSystemComponent.SetFloatParameter` (`self.NS_WaterPump`) "WaterStreamWidthPercentage" (`self.WaterStreamWidthPercentage`))
    (if (`self.AddPuddle`)
      (`SceneComponent.K2_SetWorldLocation` (`self.PuddleDecal`) _location false false)
      (else
        (`ActorComponent.K2_DestroyComponent` (`self.PuddleDecal`))))))
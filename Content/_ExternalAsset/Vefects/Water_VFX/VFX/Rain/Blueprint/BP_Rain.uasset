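; Rain VFX actor that shows falling drops and ground splashes in a zone around itself, optionally following the player camera.
; The construction script picks Niagara drops or a cheap material-driven mesh, and flat-ground or traced splashes, destroying unused components.
; Flat-ground splashes follow a single trace below the camera each Tick.
; Otherwise, rate-scaled random disc traces with frame-time holdover feed hit locations and normals to Niagara through array parameters.
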(event `self.ReceiveTick`
  (params (DeltaSeconds :type "Float (single-precision)"))
  (set `self.Delta Seconds` DeltaSeconds)
  (if (`self.Stick To Player ?`)
    (`self.StickToPlayer`))
  (if (`self.Spawn Splashes on Flat Ground Only ?`)
    (`self.SetGroundSplashes`)
    (else
      (`self.SpawnSplashes`))))

(event `StickToPlayer`
  (`self.K2_SetActorLocation` (`PlayerCameraManager.GetCameraLocation` (`GameplayStatics.GetPlayerCameraManager` 0))))

(event `SetGroundSplashes`
  (bind _returnvalue (`PlayerCameraManager.GetCameraLocation` (`GameplayStatics.GetPlayerCameraManager` 0)))
  (bind (_outhit _returnvalue_2) (`KismetSystemLibrary.LineTraceSingle` _returnvalue (- _returnvalue (`KismetMathLibrary.MakeVector` 0.0 0.0 (`self.distanceToRayTraceBelowPlayerToFindGround`))) "TraceTypeQuery1"))
  (if _returnvalue_2
    (bind _output_get (set `self.groundLocationBelowPlayer` (`.Location` (`GameplayStatics.BreakHitResult` _outhit))))
    (`SceneComponent.K2_SetWorldLocation` (`self.NS_RainSplashes_FlatGround`) _output_get false false)))

(event `SpawnSplashes`
  (bind (_returnvalue_x _returnvalue_y _returnvalue_z) (`KismetMathLibrary.BreakVector` (`self.K2_GetActorLocation`)))
  (bind _returnvalue (`KismetMathLibrary.MultiplyByPi` (* (`KismetMathLibrary.RandomFloat`) 2.0)))
  (bind _returnvalue_2 (* (`KismetMathLibrary.Sqrt` (`KismetMathLibrary.RandomFloat`)) (`self.Rain Zone Radius`)))
  (bind _returnvalue_3 (`KismetMathLibrary.MakeVector` (+ (* _returnvalue_2 (`KismetMathLibrary.Cos` _returnvalue)) _returnvalue_x) (+ (* _returnvalue_2 (`KismetMathLibrary.Sin` _returnvalue)) _returnvalue_y) (+ _returnvalue_z (`self.Rain Fall Height`))))
  (set `self.splashesToSpawnThisFrame` 0)
  (`KismetArrayLibrary.Array_Clear` (`self.splashesLocationArray`))
  (`KismetArrayLibrary.Array_Clear` (`self.splashesHitNormalArray`))
  (bind _output_get (set `self.DeltaSecondsHoldover` (+ (`self.DeltaSecondsHoldover`) (`self.Delta Seconds`))))
  (bind _returnvalue_4 (* _output_get (* (`self.Rain Fall Rate`) (/ (`self.Rain Zone Radius`) 1000.0))))
  (set `self.splashesToTrySpawningThisFrame` _returnvalue_4)
  (if (> _returnvalue_4 1.0)
    (set `self.DeltaSecondsHoldover` 0.0)
    (for _ (range 1 (+ (`KismetMathLibrary.FTrunc` (`self.splashesToTrySpawningThisFrame`)) 1))
      (bind (_outhit _returnvalue_5) (`KismetSystemLibrary.LineTraceSingle` :`Start` _returnvalue_3 :`End` (- _returnvalue_3 (`KismetMathLibrary.MakeVector` 0.0 0.0 (* (`self.Rain Fall Height`) 2.0))) :`TraceChannel` "TraceTypeQuery1" :`DrawTime` 0.1))
      (if _returnvalue_5
        (bind (_bblockinghit _binitialoverlap _time _distance _location _impactpoint _normal _impactnormal) (`GameplayStatics.BreakHitResult` _outhit))
        (`KismetArrayLibrary.Array_Add` (`self.splashesLocationArray`) _location)
        (`KismetArrayLibrary.Array_Add` (`self.splashesHitNormalArray`) _impactnormal)
        (`/Engine/EditorBlueprintResources/StandardMacros.IncrementInt` (`self.splashesToSpawnThisFrame`))))
    (`FXSystemComponent.SetIntParameter` (`self.NS_RainSplashes`) "SplashesToSpawnThisFrame" (`self.splashesToSpawnThisFrame`))
    (`NiagaraDataInterfaceArrayFunctionLibrary.SetNiagaraArrayVector` (`self.NS_RainSplashes`) "SplashesLocation" (`self.splashesLocationArray`))
    (`NiagaraDataInterfaceArrayFunctionLibrary.SetNiagaraArrayVector` (`self.NS_RainSplashes`) "SplashesHitNormal" (`self.splashesHitNormalArray`))
    (else
      (`FXSystemComponent.SetIntParameter` (`self.NS_RainSplashes`) "SplashesToSpawnThisFrame" 0))))

(fn `UserConstructionScript`
  (if (`self.Use Cheap Rain ?`)
    (`ActorComponent.K2_DestroyComponent` (`self.NS_RainDrops`))
    (bind _returnvalue (`PrimitiveComponent.CreateDynamicMaterialInstance` (`self.SM_VFX_Raindrops_Mesh`) 0 null "None"))
    (bind _output_get (set `self.CheapRainDynamicMaterialInstance` _returnvalue))
    (`MaterialInstanceDynamic.SetScalarParameterValue` _output_get "DropHeight" (`self.Rain Fall Height`))
    (`MaterialInstanceDynamic.SetScalarParameterValue` _output_get "TimeMult" (/ (`self.Rain Fall Height`) 1500.0))
    (`StaticMeshComponent.SetStaticMesh` (`self.SM_VFX_Raindrops_Mesh`) (`self.Cheap Rain Static Mesh`))
    (else
      (`ActorComponent.K2_DestroyComponent` (`self.SM_VFX_Raindrops_Mesh`))
      (`FXSystemComponent.SetFloatParameter` (`self.NS_RainDrops`) "FallHeight" (`self.Rain Fall Height`))
      (`FXSystemComponent.SetFloatParameter` (`self.NS_RainDrops`) "Radius" (`self.Rain Zone Radius`))
      (`FXSystemComponent.SetFloatParameter` (`self.NS_RainDrops`) "SpawnRate" (`self.Rain Fall Rate`))))
  (if (`self.Spawn Splashes on Flat Ground Only ?`)
    (`FXSystemComponent.SetFloatParameter` (`self.NS_RainSplashes_FlatGround`) "SpawnRate" (`self.Rain Fall Rate`))
    (`ActorComponent.K2_DestroyComponent` (`self.NS_RainSplashes`))
    (else
      (`FXSystemComponent.SetFloatParameter` (`self.NS_RainSplashes`) "SpawnRate" (`self.Rain Fall Rate`))
      (`ActorComponent.K2_DestroyComponent` (`self.NS_RainSplashes_FlatGround`)))))
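; Fire sprinkler VFX actor whose water stream and fire alarm audio toggle with the F key.
; Tick ramps StreamStrength up quickly or down more slowly, feeds it to the stream mesh's dynamic material, and collapses the mesh's X/Y scale at zero strength.
; Turning on plays a cast sound, then a delayed loop; turning off plays an end sound and fades the loop out.
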(event `self.ReceiveTick`
  (params (DeltaSeconds :type "Float (single-precision)"))
  (bind _streamscale (`self.StreamScale`))
  (bind _returnvalue (* _streamscale (`self.NormalizedScale`)))
  (set `self.Delta Seconds` DeltaSeconds)
  (if (`self.isTurnedOn?`)
    (set `self.StreamStrength` (`KismetMathLibrary.FClamp` (+ (`self.StreamStrength`) (* (`self.Delta Seconds`) 10.0))))
    (else
      (set `self.StreamStrength` (`KismetMathLibrary.FClamp` (- (`self.StreamStrength`) (* (`self.Delta Seconds`) 1.0))))))
  (`SceneComponent.SetRelativeScale3D` (`self.SM_VFX_FireSprinklerStream`) (`KismetMathLibrary.MakeVector` _returnvalue _returnvalue _streamscale))
  (`MaterialInstanceDynamic.SetScalarParameterValue` (`self.FireSprinklerStreamDynamicMaterialInstance`) "StreamStrength" (`self.StreamStrength`))
  (if (<= (`self.StreamStrength`) 0.0)
    (set `self.NormalizedScale` 0.0)
    (else
      (set `self.NormalizedScale` 1.0))))

(event `Key|F`
  (params (Key :type "Key Structure"))
  (bind _sfx_vefects_water_fire_alarm_loop_cue (`self.SFX_Vefects_Water_Fire_Alarm_Loop_Cue`))
  (:`Pressed`
    (if (`self.isTurnedOn?`)
      (set `self.isTurnedOn?` false)
      (`AudioComponent.Play` (`self.SFX_Vefects_Water_Fire_Alarm_End_Cue`) 0.0)
      (`AudioComponent.FadeOut` _sfx_vefects_water_fire_alarm_loop_cue 0.5 0.0 "Linear")
      (else
        (set `self.isTurnedOn?` true)
        (`AudioComponent.Play` (`self.SFX_Vefects_Water_Fire_Alarm_Cast_Cue`) 0.0)
        (`KismetSystemLibrary.Delay` 1.0)
        (`AudioComponent.Play` _sfx_vefects_water_fire_alarm_loop_cue 0.0)))))

(fn `UserConstructionScript`
  (`SceneComponent.SetRelativeScale3D` (`self.SM_VFX_FireSprinklerStream`) (`KismetMathLibrary.Conv_DoubleToVector` (`self.StreamScale`)))
  (bind _returnvalue (`PrimitiveComponent.CreateDynamicMaterialInstance` (`self.SM_VFX_FireSprinklerStream`) 0 null "None"))
  (set `self.FireSprinklerStreamDynamicMaterialInstance` _returnvalue))
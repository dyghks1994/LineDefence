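; Sprinkler VFX actor that toggles on and off with the K key.
; Tick ramps an on-progress value that drives the Erosion parameter on the stream and sheet dynamic materials and eases the stream's vertical scale.
; While on, the stream mesh spins around its yaw axis.
; Toggling plays cast and end sounds, starts the loop after a delay, and fades it out on shutoff.
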(event `self.ReceiveBeginPlay`
  (bind _returnvalue (`PrimitiveComponent.CreateDynamicMaterialInstance` (`self.SM_SprinklerStream`) 0 null "None"))
  (set `self.SprinklerStreamDynamicMaterialInstance` _returnvalue)
  (bind _returnvalue_2 (`PrimitiveComponent.CreateDynamicMaterialInstance` (`self.SM_VFX_SprinklerSheet`) 0 null "None"))
  (set `self.SprinklerSheetDynamicMaterialInstance` _returnvalue_2))

(event `self.ReceiveTick`
  (params (DeltaSeconds :type "Float (single-precision)"))
  (bind _streamscale (`self.StreamScale`))
  (set `self.Delta Seconds` DeltaSeconds)
  (if (`self.isTurnedOn?`)
    (set `self.OnProgress` (`KismetMathLibrary.FClamp` (+ (`self.OnProgress`) (* (`self.OnProgressRate`) (`self.Delta Seconds`)))))
    (bind _output_get (set `self.CurrentRotation` (mod (+ (`self.CurrentRotation`) (* (`self.RotationRate`) (`self.Delta Seconds`))) 1.0)))
    (`SceneComponent.K2_SetRelativeRotation` (`self.SM_SprinklerStream`) (`KismetMathLibrary.MakeRotator` 0.0 0.0 (* _output_get 360.0)) false false)
    (else
      (set `self.OnProgress` (`KismetMathLibrary.FClamp` (- (`self.OnProgress`) (* (`self.OnProgressRate`) (`self.Delta Seconds`)))))))
  (`MaterialInstanceDynamic.SetScalarParameterValue` (`self.SprinklerStreamDynamicMaterialInstance`) "Erosion" (- 1.0 (`self.OnProgress`)))
  (`MaterialInstanceDynamic.SetScalarParameterValue` (`self.SprinklerSheetDynamicMaterialInstance`) "Erosion" (- 1.0 (`self.OnProgress`)))
  (`SceneComponent.SetRelativeScale3D` (`self.SM_SprinklerStream`) (`KismetMathLibrary.MakeVector` _streamscale _streamscale (* (- 1.0 (`KismetMathLibrary.MultiplyMultiply_FloatFloat` (- 1.0 (`self.OnProgress`)) 5.0)) (`self.StreamScale`)))))

(event `Key|K`
  (params (Key :type "Key Structure"))
  (bind _sfx_vefects_water_farming_sprinkler_loop_cue (`self.SFX_Vefects_Water_Farming_Sprinkler_Loop_Cue`))
  (:`Pressed`
    (if (`self.isTurnedOn?`)
      (set `self.isTurnedOn?` false)
      (`AudioComponent.Play` (`self.SFX_Vefects_Water_Farming_Sprinkler_End_Cue`) 0.0)
      (`AudioComponent.FadeOut` _sfx_vefects_water_farming_sprinkler_loop_cue 0.5 0.0 "Linear")
      (else
        (set `self.isTurnedOn?` true)
        (`AudioComponent.Play` (`self.SFX_Vefects_Water_Farming_Sprinkler_Cast_Cue`) 0.0)
        (`KismetSystemLibrary.Delay` 1.0)
        (`AudioComponent.Play` _sfx_vefects_water_farming_sprinkler_loop_cue 0.0)))))

(fn `UserConstructionScript`
  (bind _streamscale (`self.StreamScale`))
  (`SceneComponent.SetRelativeScale3D` (`self.SM_SprinklerStream`) (`KismetMathLibrary.MakeVector` _streamscale _streamscale _streamscale)))
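; Interactive faucet VFX actor, toggled with E, that fills a sink and overflows onto the floor with a growing puddle.
; Tick drives fill level and optional draining, rescaling the stream, water plane and puddle decal to match.
; Timelines animate stream toggling and fade overflow mesh and decal through dynamic material parameters, alongside Niagara splashes and cast/loop audio.
; Construction script fits components to configurable sink dimensions and floor distance.
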(event `self.ReceiveBeginPlay`
  ;[1 1 1] INITIALIZATION
  (set `self.PuddleScale` (`self.InitialPuddleScale`))
  (if (< (`self.SinkFullness`) 1.0)
    (`SceneComponent.SetVisibility` (`self.OverflowMesh`) false false)
    (`ActorComponent.Deactivate` (`self.NS_Splash_Floor_From_Overflowed_Sink`)))
  (bind _returnvalue (`DecalComponent.CreateDynamicMaterialInstance` (`self.PuddleDecal`)))
  (set `self.PuddleDecalDynamicMaterialInstance` _returnvalue)
  (if (`self.StartWithFaucetTurnedOn?`)
    (set `self.isFaucetOn?` true)
    (bind _returnvalue_2 (`PrimitiveComponent.CreateDynamicMaterialInstance` (`self.OverflowMesh`) 0 null "None"))
    (set `self.OverflowMeshDynamicMaterialInstance` _returnvalue_2)
    (else
      (set `self.SinkFullness` 0.0)
      (`SceneComponent.SetVisibility` (`self.OverflowMesh`) false false)
      (bind _returnvalue_3 (`PrimitiveComponent.CreateDynamicMaterialInstance` (`self.OverflowMesh`) 0 null "None"))
      (set `self.OverflowMeshDynamicMaterialInstance` _returnvalue_3)
      (`SceneComponent.SetVisibility` (`self.WaterPlane`) false false)
      (`ActorComponent.Deactivate` (`self.NS_Splash_Sink`))
      (`ActorComponent.Deactivate` (`self.NS_Splash_Floor_From_Overflowed_Sink`))
      (set `self.WaterStreamScalePercentageNormalized` 0.0)
      (set `self.isFaucetOn?` false))))

(event `self.ReceiveTick`
  (params (DeltaSeconds :type "Float (single-precision)"))
  ;[1 1 1] TICK BEHAVIOR
  (set `self.Delta Seconds` DeltaSeconds)
  (`self.UpdateWaterElements`)
  (if (`self.isFaucetOn?`)
    (if (< (`self.SinkFullness`) 1.0)
      (set `self.SinkFullness` (`KismetMathLibrary.FClamp` (+ (`self.SinkFullness`) (* (`self.Delta Seconds`) (`self.FaucetFlowRate`)))))
      (else
        (set `self.PuddleScale` (`KismetMathLibrary.FClamp` (+ (`self.PuddleScale`) (* (`self.Delta Seconds`) (`self.PuddleScaleRate`)))))
        (if (not (`self.isOverflowing?`))
          (`self.StartOverflow`))))
    (elif (`self.DrainWaterWhenFaucetIsTurnedOff`)
      (set `self.SinkFullness` (`KismetMathLibrary.FClamp` (- (`self.SinkFullness`) (* (`self.Delta Seconds`) (`self.FaucetFlowRate`)))))
      (if (`self.isOverflowing?`)
        (`self.StopOverflow`)))))

(event `StartOverflow`
  ;[1 1 1] OVERFLOW
  (set `self.isOverflowing?` true)
  (`SceneComponent.SetVisibility` (`self.OverflowMesh`) true false)
  (`ActorComponent.Activate` (`self.NS_Splash_Floor_From_Overflowed_Sink`) false)
  (`|ExecutionSequence`
    (:`then_0`
      (bind (_direction _newtrack_0 _newtrack_1) (`Timeline|FadeInOverflowMesh` :!via `PlayFromStart`)
        (:`Update`
          (`MaterialInstanceDynamic.SetScalarParameterValue` (`self.OverflowMeshDynamicMaterialInstance`) "RefractionStrength" _newtrack_0)
          (`MaterialInstanceDynamic.SetScalarParameterValue` (`self.PuddleDecalDynamicMaterialInstance`) "ErodeIn" _newtrack_1)
          (`MaterialInstanceDynamic.SetScalarParameterValue` (`self.PuddleDecalDynamicMaterialInstance`) "ErodeOut" 0.0))))
    (:`then_1`
      (`AudioComponent.Play` (`self.SFX_Vefects_Water_Faucet_Waterfall_Cast_Cue`) 0.0)
      (`KismetSystemLibrary.Delay` 1.0)
      (`AudioComponent.Play` (`self.SFX_Vefects_Water_Faucet_Waterfall_Loop_Cue`) 0.0))))

(event `StopOverflow`
  ;[1 1 1] OVERFLOW
  (set `self.isOverflowing?` false)
  (`ActorComponent.Deactivate` (`self.NS_Splash_Floor_From_Overflowed_Sink`))
  (`|ExecutionSequence`
    (:`then_0`
      (bind (_direction _newtrack_0) (`Timeline|FadeOutOverflowMesh` :!via `PlayFromStart`)
        (:`Update`
          (`MaterialInstanceDynamic.SetScalarParameterValue` (`self.OverflowMeshDynamicMaterialInstance`) "RefractionStrength" _newtrack_0)
          (`MaterialInstanceDynamic.SetScalarParameterValue` (`self.PuddleDecalDynamicMaterialInstance`) "ErodeOut" (- 1.0 _newtrack_0)))
        (:`Finished`
          (`SceneComponent.SetVisibility` (`self.OverflowMesh`) false false))))
    (:`then_1`
      (`AudioComponent.FadeOut` (`self.SFX_Vefects_Water_Faucet_Waterfall_Loop_Cue`) 1.0 0.0 "Linear"))))

(event `Key|E`
  (params (Key :type "Key Structure"))
  ;[1 1 1] CONTROLS
  (:`Pressed`
    (if (`self.isFaucetOn?`)
      (`self.TurnFaucentOff`)
      (else
        (`self.TurnFaucetOn`)))))

(event `TurnFaucetOn`
  ;[1 1 1] CONTROLS
  (if (`self.canInteractWithFaucet?`)
    (set `self.canInteractWithFaucet?` false)
    (`|ExecutionSequence`
      (:`then_0`
        (bind (_direction _newtrack_0) (`Timeline|WaterStreamTurningOn` :!via `PlayFromStart`)
          (:`Update`
            (set `self.WaterStreamScalePercentageNormalized` _newtrack_0))
          (:`Finished`
            (set `self.isFaucetOn?` true)
            (`ActorComponent.Activate` (`self.NS_Splash_Sink`) false)
            (set `self.canInteractWithFaucet?` true))))
      (:`then_1`
        (`AudioComponent.Play` (`self.SFX_Vefects_Water_Faucet_Surface_Cast_Cue`) 0.0)
        (`KismetSystemLibrary.Delay` 1.0)
        (`AudioComponent.Play` (`self.SFX_Vefects_Water_Faucet_Surface_Loop_Cue`) 0.0)))))

(event `TurnFaucentOff`
  ;[1 1 1] CONTROLS
  (if (`self.canInteractWithFaucet?`)
    (set `self.canInteractWithFaucet?` false)
    (`|ExecutionSequence`
      (:`then_0`
        (bind (_direction _newtrack_0) (`Timeline|WaterStreamTurningOff` :!via `PlayFromStart`)
          (:`Update`
            (set `self.WaterStreamScalePercentageNormalized` _newtrack_0))
          (:`Finished`
            (set `self.isFaucetOn?` false)
            (`ActorComponent.Deactivate` (`self.NS_Splash_Sink`))
            (set `self.canInteractWithFaucet?` true))))
      (:`then_1`
        (`AudioComponent.FadeOut` (`self.SFX_Vefects_Water_Faucet_Surface_Loop_Cue`) 1.0 0.0 "Linear")))))

(fn `InitializeWaterElements`
  (bind (_sinkdimensions_x _sinkdimensions_y _sinkdimensions_z) (`KismetMathLibrary.BreakVector` (`self.SinkDimensions`)))
  (bind _sinkdimensions_x_2 (`KismetMathLibrary.BreakVector` (`self.SinkDimensions`)))
  (bind (_sinkdimensions_x_3 _sinkdimensions_y_2) (`KismetMathLibrary.BreakVector` (`self.SinkDimensions`)))
  (bind (_sinkdimensions_x_4 _sinkdimensions_y_3) (`KismetMathLibrary.BreakVector` (`self.SinkDimensions`)))
  (bind (_origin _boxextent) (`KismetSystemLibrary.GetComponentBounds` (`self.OverflowMesh`)))
  (bind (_returnvalue_x _returnvalue_y _returnvalue_z) (`KismetMathLibrary.BreakVector` (+ (`self.SinkOffset`) (`KismetMathLibrary.MakeVector` 0.0 0.0 _sinkdimensions_z))))
  (bind _returnvalue (+ _origin (`KismetMathLibrary.MakeVector` 0.0 (/ (.y _boxextent) 2.0) (* (.z _boxextent) -1.0))))
  (`SceneComponent.SetRelativeScale3D` (`self.WaterPlane`) (`KismetMathLibrary.MakeVector` (/ _sinkdimensions_x_4 100.0) (/ _sinkdimensions_y_3 100.0) 1.0))
  (`SceneComponent.K2_SetRelativeLocation` (`self.OverflowMesh`) (`KismetMathLibrary.MakeVector` 0.0 (`self.SinkBorderOffset`) (+ _returnvalue_z 1.0)) false false)
  (`NiagaraComponent.SetVariableFloat` (`self.NS_Splash_Floor_From_Overflowed_Sink`) "Width" (+ _sinkdimensions_y_2 15.0))
  (`SceneComponent.SetRelativeScale3D` (`self.OverflowMesh`) (`KismetMathLibrary.MakeVector` (/ _sinkdimensions_x_2 100.0) 1.0 (* (`self.OverflowMeshZScalePercentageNormalized`) (/ (`self.DistanceFromSinkTopToFloor`) 100.0))))
  (`SceneComponent.K2_SetWorldLocation` (`self.NS_Splash_Floor_From_Overflowed_Sink`) _returnvalue false false)
  (`SceneComponent.K2_SetWorldLocation` (`self.PuddleDecal`) _returnvalue false false))

(fn `UpdateWaterElements`
  (bind _waterstreamscalepercentagenormalized (`self.WaterStreamScalePercentageNormalized`))
  (bind (_sinkdimensions_x _sinkdimensions_y _sinkdimensions_z) (`KismetMathLibrary.BreakVector` (`self.SinkDimensions`)))
  (bind (_sinkdimensions_x_2 _sinkdimensions_y_2 _sinkdimensions_z_2) (`KismetMathLibrary.BreakVector` (`self.SinkDimensions`)))
  (bind (_maxpuddledimensions_x _maxpuddledimensions_y) (`KismetMathLibrary.BreakVector2D` (`self.MaxPuddleDimensions`)))
  (bind _sinkdimensions_x_3 (`KismetMathLibrary.BreakVector` (`self.SinkDimensions`)))
  (bind (_sinkdimensions_x_4 _sinkdimensions_y_3 _sinkdimensions_z_3) (`KismetMathLibrary.BreakVector` (`self.SinkDimensions`)))
  (bind (_sinkoffset_x _sinkoffset_y _sinkoffset_z) (`KismetMathLibrary.BreakVector` (`self.SinkOffset`)))
  (bind (_returnvalue_x _returnvalue_y _returnvalue_z) (`KismetMathLibrary.BreakVector` (+ (`self.SinkOffset`) (`KismetMathLibrary.MakeVector` 0.0 0.0 (* (`self.SinkFullness`) _sinkdimensions_z_2)))))
  (`SceneComponent.SetRelativeScale3D` (`self.WaterStream`) (`KismetMathLibrary.MakeVector` _waterstreamscalepercentagenormalized _waterstreamscalepercentagenormalized (/ (`KismetMathLibrary.Abs` (+ _sinkoffset_z (* (`self.SinkFullness`) _sinkdimensions_z_3))) 40.0)))
  (`SceneComponent.K2_SetRelativeLocation` (`self.WaterPlane`) (+ (`self.SinkOffset`) (`KismetMathLibrary.MakeVector` 0.0 0.0 (* (`self.SinkFullness`) _sinkdimensions_z))) false false)
  (`SceneComponent.K2_SetRelativeLocation` (`self.NS_Splash_Sink`) (`KismetMathLibrary.MakeVector` 0.0 0.0 _returnvalue_z) false false)
  (`SceneComponent.SetRelativeScale3D` (`self.OverflowMesh`) (`KismetMathLibrary.MakeVector` (/ _sinkdimensions_x_3 100.0) 1.0 (* (`self.OverflowMeshZScalePercentageNormalized`) (/ (`self.DistanceFromSinkTopToFloor`) 100.0))))
  (`SceneComponent.SetRelativeScale3D` (`self.PuddleDecal`) (`KismetMathLibrary.MakeVector` 1.0 (* (/ _maxpuddledimensions_x 256.0) (`self.PuddleScale`)) (* (/ _maxpuddledimensions_y 256.0) (`self.PuddleScale`))))
  (if (<= (`self.SinkFullness`) 0.0)
    (`SceneComponent.SetVisibility` (`self.WaterPlane`) false false)
    (else
      (`SceneComponent.SetVisibility` (`self.WaterPlane`) true false))))

(fn `UserConstructionScript`
  (`self.InitializeWaterElements`)
  (`self.UpdateWaterElements`))
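; BP_Laser is a laser beam actor that the 1 key toggles on and off, along with its start and loop audio.
; Each tick it line traces forward on the Camera channel and feeds the hit or trace end to the Niagara "Beam End" variable.
; Beam length grows over time up to a cap and snaps back to any blocking hit.
; A cube component also spins with slight random variation.
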(event `self.ReceiveBeginPlay`
  (`self.EnableInput` (`GameplayStatics.GetPlayerController` 0)))

(event `self.ReceiveTick`
  (params (DeltaSeconds :type "Float (single-precision)"))
  (bind _returnvalue (`self.K2_GetActorLocation`))
  (bind _returnvalue_2 (+ _returnvalue (* (`self.GetActorForwardVector`) (`self.Distance`))))
  (`|ExecutionSequence`
    (:`then_0`
      ;[1 1 1] Basic Laser
      (`|ExecutionSequence`
        (:`then_0`
          (`SceneComponent.K2_AddWorldRotation` (`self.Cube`) (`KismetMathLibrary.MakeRotator` (`KismetMathLibrary.RandomFloatInRange` -0.05 -0.16)) false false))
        (:`then_1`
          (set `self.TraceEnd` _returnvalue_2)
          (bind _outhit (`KismetSystemLibrary.LineTraceSingle` _returnvalue _returnvalue_2 "TraceTypeQuery2"))
          (`NiagaraComponent.SetVariableVec3` (`self.NS_Laser`) "Beam End" (select `bool` (`GameplayStatics.BreakHitResult` _outhit) :`false` (`self.TraceEnd`) :`true` (`.Location` (`GameplayStatics.BreakHitResult` _outhit))))
          (if (`GameplayStatics.BreakHitResult` _outhit)
            (set `self.Distance` (`KismetMathLibrary.VSize` (- (`.Location` (`GameplayStatics.BreakHitResult` _outhit)) (`self.K2_GetActorLocation`))))))))
    (:`then_1`
      (if (< (`self.Distance`) 20000.0)
        (set `self.Distance` (+ (`self.Distance`) (* DeltaSeconds (`self.LaserFirstLengthSpeed`))))))))

(event `Key|One`
  (params (Key :type "Key Structure"))
  (:`Pressed`
    (`/Engine/EditorBlueprintResources/StandardMacros.FlipFlop`
      (:`A`
        (bind _returnvalue (`AddComponent|NODE_AddAudioComponent-0`))
        (set `self.Audio_Start` _returnvalue)
        (bind _returnvalue_2 (`AddComponent|NODE_AddAudioComponent-1`))
        (set `self.Audio_Loop` _returnvalue_2)
        (`ActorComponent.SetActive` (`self.NS_Laser`) true false))
      (:`B`
        (`ActorComponent.Deactivate` (`self.NS_Laser`))
        (`AudioComponent.Stop` _returnvalue)
        (`AudioComponent.Stop` _returnvalue_2)))))

(fn `UserConstructionScript`)